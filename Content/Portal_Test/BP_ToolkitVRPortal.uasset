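; VR portal actor that shows a stereo view from a linked target portal and, when DebugBool is set, teleports the player through.
; Two scene captures, offset by pupil distance, render into viewport-sized targets feeding the other portal's hemisphere material.
; While active, Tick mirrors the camera's portal-relative transform onto the target's capture rig; crossing moves the pawn likewise and closes both portals.
; A reversible timeline animates ring radii and toggles the hemisphere.
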(event Custom|ActivatePortal
  (bind _portalhemisphere (Variables|Default|GetPortalHemisphere))
  (bind _portalring (Variables|Default|GetPortalRing))
  (bind (_direction _outerring _innerring) (Timeline|PortalActivateTimeline Play)
    (:Update
      (Rendering|Material|SetScalarParameterValue _portalring "OuterRadius" (Math|Float|Lerp -0.02 0.3 _outerring) :!class /Script/Engine.MaterialInstanceDynamic)
      (Rendering|Material|SetScalarParameterValue _portalring "InnerRadius" (Math|Float|Lerp -0.2 0.25 _innerring) :!class /Script/Engine.MaterialInstanceDynamic))
    (:HidePortalHemisphere
      (switch Utilities|FlowControl|Switch|SwitchonETimelineDirection _direction
        (:Forward
          (Rendering|SetVisibility _portalhemisphere true false)
          (Variables|Default|SetbIsPortalActivated true))
        (:Backward
          (Rendering|SetVisibility _portalhemisphere false false)
          (Variables|Default|SetbIsPortalActivated false))))))

(event Custom|DeactivatePortal
  (bind _portalhemisphere (Variables|Default|GetPortalHemisphere))
  (bind _portalring (Variables|Default|GetPortalRing))
  (bind (_direction _outerring _innerring) (Timeline|PortalActivateTimeline Reverse)
    (:Update
      (Rendering|Material|SetScalarParameterValue _portalring "OuterRadius" (Math|Float|Lerp -0.02 0.3 _outerring) :!class /Script/Engine.MaterialInstanceDynamic)
      (Rendering|Material|SetScalarParameterValue _portalring "InnerRadius" (Math|Float|Lerp -0.2 0.25 _innerring) :!class /Script/Engine.MaterialInstanceDynamic))
    (:HidePortalHemisphere
      (switch Utilities|FlowControl|Switch|SwitchonETimelineDirection _direction
        (:Forward
          (Rendering|SetVisibility _portalhemisphere true false)
          (Variables|Default|SetbIsPortalActivated true))
        (:Backward
          (Rendering|SetVisibility _portalhemisphere false false)
          (Variables|Default|SetbIsPortalActivated false))))))

(event EventBeginPlay
  (bind _returnvalue (Game|GetPlayerController 0))
  (bind _portalring (Variables|Default|GetPortalRing))
  (bind (_sizex _sizey) (HUD|GetViewportSize _returnvalue))
  (Utilities|FlowControl|Sequence
    (:then_0
      (CallFunction|CreateRenderCapture _sizex _sizey))
    (:then_1
      (bind _returnvalue_2 (AddComponent|AddSceneCaptureComponent2D true))
      (bind _output_get (Variables|Default|SetRenderCaptureLeft _returnvalue_2))
      (Transformation|AttachComponentToComponent _output_get (Variables|Default|GetRenderCaptureRoot) "None" "SnapToTarget" "SnapToTarget" "SnapToTarget" true)
      (Transformation|SetRelativeLocation _output_get (Math|Vector|MakeVector 0.0 (* (Variables|Default|GetPupilDistance) -0.5) 0.0) false false)
      (Variables|/Script/Engine.SceneCaptureComponent|SetCaptureSource _output_get "SCS_SceneColorHDRNoAlpha")
      (Variables|/Script/Engine.SceneCaptureComponent|SetbCaptureEveryFrame _output_get true)
      (Components|Tick|SetTickGroup _output_get "TG_PostPhysics"))
    (:then_2
      (bind _returnvalue_3 (AddComponent|AddSceneCaptureComponent2D true))
      (bind _output_get_2 (Variables|Default|SetRenderCaptureRight _returnvalue_3))
      (Transformation|AttachComponentToComponent _output_get_2 (Variables|Default|GetRenderCaptureRoot) "None" "KeepRelative" "KeepRelative" "KeepRelative" true)
      (Transformation|SetRelativeLocation _output_get_2 (Math|Vector|MakeVector 0.0 (* (Variables|Default|GetPupilDistance) 0.5) 0.0) false false)
      (Variables|/Script/Engine.SceneCaptureComponent|SetCaptureSource _output_get_2 "SCS_SceneColorHDRNoAlpha")
      (Variables|/Script/Engine.SceneCaptureComponent|SetbCaptureEveryFrame _output_get_2 true)
      (Components|Tick|SetTickGroup _output_get_2 "TG_PostPhysics"))
    (:then_3
      (Components|Tick|SetTickGroup "TG_PostUpdateWork"))
    (:then_4
      (Utilities|FlowControl|Delay 0.2)
      (bind _targetportal (Variables|Default|GetTargetPortal)
        (:then
          (bind (_left _right) (CallFunction|GetRenderCapture _targetportal))
          (Variables|/Script/Engine.SceneCaptureComponent2D|SetTextureTarget _left (Variables|Default|GetRenderLeft))
          (Variables|/Script/Engine.SceneCaptureComponent2D|SetTextureTarget _right (Variables|Default|GetRenderRight)))
        (:else)))
    (:then_5
      (Rendering|SetVisibility (Variables|Default|GetPortalHemisphere) false false)
      (Rendering|Material|SetScalarParameterValue _portalring "OuterRadius" -0.02 :!class /Script/Engine.MaterialInstanceDynamic)
      (Rendering|Material|SetScalarParameterValue _portalring "InnerRadius" -0.2 :!class /Script/Engine.MaterialInstanceDynamic))))

(event EventTick
  (params (DeltaSeconds :type Float%20%28single-precision%29))
  (bind _returnvalue (Game|GetPlayerCameraManager 0))
  (bind _returnvalue_2 (Transformation|GetActorTransform))
  (bind _returnvalue_3 (Game|Player|GetPlayerPawn 0))
  (bind _returnvalue_4 (Transformation|GetActorTransform))
  (bind _targetportal (Variables|Default|GetTargetPortal))
  (bind _returnvalue_5 (Transformation|GetActorLocation _returnvalue))
  (bind _returnvalue_6 (Transformation|GetActorTransform _targetportal))
  (bind _returnvalue_7 (Math|Transform|InverseTransformLocation _returnvalue_4 _returnvalue_5))
  (if (Variables|Default|GetbIsPortalActivated)
    (bind _targetportal_2 (Variables|Default|GetTargetPortal)
      (:then
        (CallFunction|UpdateRenderCapture _targetportal_2 _returnvalue_7 (Math|Transform|InverseTransformRotation _returnvalue_4 (Transformation|GetActorRotation _returnvalue)))
        (if (not (> (.X (Math|Vector|BreakVector _returnvalue_7)) -2e+01))
          (if (Variables|Default|GetDebugBool)
            (Transformation|SetActorLocationAndRotation _returnvalue_3 (Math|Transform|TransformLocation _returnvalue_6 (Math|Transform|InverseTransformLocation _returnvalue_2 (Transformation|GetActorLocation _returnvalue_3))) (Math|Transform|TransformRotation _returnvalue_6 (Math|Transform|InverseTransformRotation _returnvalue_2 (Transformation|GetActorRotation _returnvalue_3))) false true)
            (CallFunction|DeactivatePortal (Variables|Default|GetTargetPortal)))))
      (:else))))

(fn ConstructionScript
  (Transformation|SetRelativeRotation (Variables|Default|GetPortalHemisphere) (Math|Rotator|MakeRotator 0.0 0.0 (Math|Float|SelectFloat 1.8e+02 0.0 (Variables|Default|GetbInversePortal))) false false)
  (bind _returnvalue (Rendering|Material|CreateDynamicMaterialInstance (Variables|Default|GetPortalRingPlane) 0 "/Game/Portal_Test/MI_PortalRing.MI_PortalRing" "None" :!class /Script/Engine.PrimitiveComponent))
  (Variables|Default|SetPortalRing _returnvalue)
  (bind _returnvalue_2 (Rendering|Material|CreateDynamicMaterialInstance (Variables|Default|GetPortalHemisphere) 0 "/Game/Portal_Test/M_PortalRender.M_PortalRender" "None" :!class /Script/Engine.PrimitiveComponent))
  (Variables|Default|SetPortalRender _returnvalue_2))

(fn GetRenderCapture
  (return (Variables|Default|GetRenderCaptureLeft) (Variables|Default|GetRenderCaptureRight)))

(fn UpdateRenderCapture
  (params (Location :type Vector) (Rotation :type Rotator))
  (Transformation|SetRelativeLocationAndRotation (Variables|Default|GetRenderCaptureRoot) Location Rotation false false))

(fn CreateRenderCapture
  (params (Width :type Integer) (Height :type Integer))
  (bind _returnvalue (Rendering|CreateRenderTarget2D Width Height "RTF_RGBA16f"))
  (bind _output_get (Variables|Default|SetRenderLeft _returnvalue))
  (Rendering|Material|SetTextureParameterValue (Variables|Default|GetPortalRender) "LeftRender" _output_get)
  (bind _returnvalue_2 (Rendering|CreateRenderTarget2D Width Height "RTF_RGBA16f"))
  (bind _output_get_2 (Variables|Default|SetRenderRight _returnvalue_2))
  (Rendering|Material|SetTextureParameterValue (Variables|Default|GetPortalRender) "RightRender" _output_get_2))
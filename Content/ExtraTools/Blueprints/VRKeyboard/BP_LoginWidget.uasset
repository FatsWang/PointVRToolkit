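; VR login panel actor that hosts a WBP_Login widget and holds the company number, account and password input.
; Three box components select the active field, by hand hover when the laser is off or by grab press when it is on.
; AddString and Delete edit the selected field's string, and a separate UpdateString event writes it to that field's text.
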(event Custom|UpdateString
  (switch Utilities|FlowControl|Switch|SwitchonE_InputTarget (Variables|Default|GetInputTarget)
    (:NewEnumerator0
      (Rendering|Components|TextRender|SetText (Variables|Default|GetCompanyNum) (Utilities|Text|ToText(String) (Variables|Default|GetStr_CompanyNum))))
    (:NewEnumerator1
      (Rendering|Components|TextRender|SetText (Variables|Default|GetAccount) (Utilities|Text|ToText(String) (Variables|Default|GetStr_Account))))
    (:NewEnumerator2
      (Rendering|Components|TextRender|SetText (Variables|Default|GetPassword) (Utilities|Text|ToText(String) (Variables|Default|GetStr_Password))))))

(event Custom|AddString
  (params (InChar :type String))
  (switch Utilities|FlowControl|Switch|SwitchonE_InputTarget (Variables|Default|GetInputTarget)
    (:NewEnumerator0
      (Variables|Default|SetStr_CompanyNum (Utilities|String|Append (Variables|Default|GetStr_CompanyNum) InChar)))
    (:NewEnumerator1
      (Variables|Default|SetStr_Account (Utilities|String|Append (Variables|Default|GetStr_Account) InChar)))
    (:NewEnumerator2
      (Variables|Default|SetStr_Password (Utilities|String|Append (Variables|Default|GetStr_Password) InChar)))))

(event Custom|Delete
  (switch Utilities|FlowControl|Switch|SwitchonE_InputTarget (Variables|Default|GetInputTarget)
    (:NewEnumerator0
      (Variables|Default|SetStr_CompanyNum (Utilities|String|LeftChop (Variables|Default|GetStr_CompanyNum) 1)))
    (:NewEnumerator1
      (Variables|Default|SetStr_Account (Utilities|String|LeftChop (Variables|Default|GetStr_Account) 1)))
    (:NewEnumerator2
      (Variables|Default|SetStr_Password (Utilities|String|LeftChop (Variables|Default|GetStr_Password) 1)))))

(event EventBeginPlay
  (bind _aswbp_login (Utilities|Casting|CastToWBP_Login (UserInterface|GetUserWidgetObject (Variables|Default|GetWidget))))
  (Variables|Default|SetWBP_Login _aswbp_login))

(fn ConstructionScript)

(fn IsInteractiveComponent
  (params (Interactor :type BPC%20Toolkit%20Motion%20Interactor%20Object%20Reference) (Component :type Primitive%20Component%20Object%20Reference))
  (return (Math|Boolean|ORBoolean (== Component (Variables|Default|GetBox)) (== Component (Variables|Default|GetBox1)) (== Component (Variables|Default|GetBox2)))))

(fn OnComponentHovered
  (params (Interactor :type BPC%20Toolkit%20Motion%20Interactor%20Object%20Reference) (HoveredComponent :type Primitive%20Component%20Object%20Reference))
  ;[1 1 1] 未使用射线时
  (bind _asbp_toolkit_vrhand (Utilities|Casting|CastToBP_ToolkitVRHand (Components|GetOwner Interactor)))
  (if (not (Variables|/Game/PointVRToolkit/Blueprints/Characters/VirtualReality/BP_ToolkitVRHand.BP_ToolkitVRHand_C|GetbIsLaserActivated _asbp_toolkit_vrhand))
    (if (== HoveredComponent (Variables|Default|GetBox))
      (Variables|Default|SetInputTarget "NewEnumerator0")
      (return false)
      (elif (== HoveredComponent (Variables|Default|GetBox1))
        (Variables|Default|SetInputTarget "NewEnumerator1")
        (return false)
        (elif (== HoveredComponent (Variables|Default|GetBox2))
          (Variables|Default|SetInputTarget "NewEnumerator2")
          (return false))))))

(fn OnComponentUnhovered
  (params (Interactor :type BPC%20Toolkit%20Motion%20Interactor%20Object%20Reference) (UnhoveredComponent :type Primitive%20Component%20Object%20Reference))
  (return false))

(fn OnDragCanceled
  (params (Interactor :type BPC%20Toolkit%20Motion%20Interactor%20Object%20Reference))
  (return false))

(fn OnDragDetected
  (params (Interactor :type BPC%20Toolkit%20Motion%20Interactor%20Object%20Reference))
  (return false))

(fn OnDragMove
  (params (Interactor :type BPC%20Toolkit%20Motion%20Interactor%20Object%20Reference))
  (return false))

(fn OnGrabPressed
  (params (Interactor :type BPC%20Toolkit%20Motion%20Interactor%20Object%20Reference))
  (bind _component (Default|GetHoveredObject Interactor))
  (bind _asbp_toolkit_vrhand (Utilities|Casting|CastToBP_ToolkitVRHand (Components|GetOwner Interactor)))
  (if (Variables|/Game/PointVRToolkit/Blueprints/Characters/VirtualReality/BP_ToolkitVRHand.BP_ToolkitVRHand_C|GetbIsLaserActivated _asbp_toolkit_vrhand)
    (if (== _component (Variables|Default|GetBox))
      (Variables|Default|SetInputTarget "NewEnumerator0")
      (return false)
      (elif (== _component (Variables|Default|GetBox1))
        (Variables|Default|SetInputTarget "NewEnumerator1")
        (return false)
        (elif (== _component (Variables|Default|GetBox2))
          (Variables|Default|SetInputTarget "NewEnumerator2")
          (return false))))))

(fn OnGrabReleased
  (params (Interactor :type BPC%20Toolkit%20Motion%20Interactor%20Object%20Reference))
  (return false))

(fn OnHoverEnter
  (params (Interactor :type BPC%20Toolkit%20Motion%20Interactor%20Object%20Reference))
  (return false))

(fn OnHoverLeave
  (params (Interactor :type BPC%20Toolkit%20Motion%20Interactor%20Object%20Reference))
  (return false))

(fn OnHoverMove
  (params (Interactor :type BPC%20Toolkit%20Motion%20Interactor%20Object%20Reference))
  (return false))

(fn OnUsePressed
  (params (Interactor :type BPC%20Toolkit%20Motion%20Interactor%20Object%20Reference))
  (return false))

(fn OnUseReleased
  (params (Interactor :type BPC%20Toolkit%20Motion%20Interactor%20Object%20Reference))
  (return false))
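; VR keyboard actor that builds its layout of key buttons in the construction script.
; Each of four row arrays spawns BP_Keyboard_Button child actor components, spaced evenly along Y.
; Successive rows step back along X and shift sideways for a staggered keyboard look.
; Every spawned button receives its array element as its content.
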(fn ConstructionScript
  (for (_array_element _array_index) (Variables|Default|GetRow1)
    (bind _returnvalue (AddComponent|AddChildActorComponent false (Math|Transform|MakeTransform (Math|Vector|MakeVector 0.0 (* _array_index 6.0) 0.0) "0, 0, 0" "1,1,1")))
    (ChildActorComponent|SetChildActorClass _returnvalue "/Game/ExtraTools/Blueprints/VRKeyboard/BP_Keyboard_Button.BP_Keyboard_Button_C")
    (bind _asbp_keyboard_button (Utilities|Casting|CastToBP_Keyboard_Button (Variables|/Script/Engine.ChildActorComponent|GetChildActor _returnvalue)))
    (Default|SetButtonContent _asbp_keyboard_button _array_element))
  (for (_array_element_2 _array_index_2) (Variables|Default|GetRow2)
    (bind _returnvalue_2 (AddComponent|AddChildActorComponent false (Math|Transform|MakeTransform (+ (Math|Vector|MakeVector -7.0 (* _array_index_2 6.0) 0.0) "0,3.000000, 0") "0, 0, 0" "1,1,1")))
    (ChildActorComponent|SetChildActorClass _returnvalue_2 "/Game/ExtraTools/Blueprints/VRKeyboard/BP_Keyboard_Button.BP_Keyboard_Button_C")
    (bind _asbp_keyboard_button_2 (Utilities|Casting|CastToBP_Keyboard_Button (Variables|/Script/Engine.ChildActorComponent|GetChildActor _returnvalue_2)))
    (Default|SetButtonContent _asbp_keyboard_button_2 _array_element_2))
  (for (_array_element_3 _array_index_3) (Variables|Default|GetRow3)
    (bind _returnvalue_3 (AddComponent|AddChildActorComponent false (Math|Transform|MakeTransform (+ (Math|Vector|MakeVector -14.0 (* _array_index_3 6.0) 0.0) "0,6.000000, 0") "0, 0, 0" "1,1,1")))
    (ChildActorComponent|SetChildActorClass _returnvalue_3 "/Game/ExtraTools/Blueprints/VRKeyboard/BP_Keyboard_Button.BP_Keyboard_Button_C")
    (bind _asbp_keyboard_button_3 (Utilities|Casting|CastToBP_Keyboard_Button (Variables|/Script/Engine.ChildActorComponent|GetChildActor _returnvalue_3)))
    (Default|SetButtonContent _asbp_keyboard_button_3 _array_element_3))
  (for (_array_element_4 _array_index_4) (Variables|Default|GetRow4)
    (bind _returnvalue_4 (AddComponent|AddChildActorComponent false (Math|Transform|MakeTransform (+ (Math|Vector|MakeVector -21.0 (* _array_index_4 6.0) 0.0) "0,9.000000, 0") "0, 0, 0" "1,1,1")))
    (ChildActorComponent|SetChildActorClass _returnvalue_4 "/Game/ExtraTools/Blueprints/VRKeyboard/BP_Keyboard_Button.BP_Keyboard_Button_C")
    (bind _asbp_keyboard_button_4 (Utilities|Casting|CastToBP_Keyboard_Button (Variables|/Script/Engine.ChildActorComponent|GetChildActor _returnvalue_4)))
    (Default|SetButtonContent _asbp_keyboard_button_4 _array_element_4)))
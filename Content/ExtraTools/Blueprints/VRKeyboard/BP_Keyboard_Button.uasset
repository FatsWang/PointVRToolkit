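; A VR keyboard key that types its text into the BP_LoginWidget found at BeginPlay, or deletes when its text is "De".
; Hover gives haptics and a glow, and finger movement pushes the key down in local Z while the hand's laser is inactive.
; Full depth fires one press with a color change until the depth drops, and grab also presses.
; Tick interpolates the key back toward rest.
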(event Custom|CheckReachedEnd
  (bind _button (Variables|Default|GetButton))
  (if (>= (Variables|Default|GetPressDepth) (Variables|Default|GetMaxPressDepth))
    (Utilities|FlowControl|DoOnce false :!label _label
      (:Completed
        (Utilities|FlowControl|Sequence
          (:then_0
            (Rendering|Material|SetVectorParameterValueonMaterials _button "BaseColor" "0,0.400000,1.000000")
            (Utilities|FlowControl|Delay 0.2)
            (Rendering|Material|SetVectorParameterValueonMaterials _button "None" "0,0.500000,1.000000"))
          (:then_1
            (CallFunction|ButtonPressed)))))
    (else
      (goto _label Reset))))

(event Custom|ButtonPressed
  (bind _loginui (Variables|Default|GetLoginUI))
  (bind _text (Variables|Default|GetText))
  (Default|CallOnButtonPressed)
  (switch string _text
    (:Default
      (Default|AddString _loginui _text))
    (:De
      (Default|Delete _loginui)))
  (Default|UpdateString _loginui))

(event Custom|SetButtonContent
  (params (Text :type String))
  (bind _output_get (Variables|Default|SetText Text))
  (Rendering|Components|TextRender|SetText (Variables|Default|GetTextContent) (Utilities|Text|ToText(String) _output_get)))

(event EventBeginPlay
  ;[1 1 1] 开始时获得按钮的初始位置
  (Variables|Default|SetButtonInitialLocation (Variables|/Script/Engine.SceneComponent|GetRelativeLocation (Variables|Default|GetButtonRoot)))
  (bind _outactors (Actor|GetAllActorsOfClass "/Game/ExtraTools/Blueprints/VRKeyboard/BP_LoginWidget.BP_LoginWidget_C"))
  (Variables|Default|SetLoginUI (Utilities|Array|Get(acopy) _outactors)))

(event EventTick
  (params (DeltaSeconds :type Float%20%28single-precision%29))
  (Transformation|SetRelativeLocation (Variables|Default|GetButtonRoot) (Math|Interpolation|VInterpTo (Variables|/Script/Engine.SceneComponent|GetRelativeLocation (Variables|Default|GetButtonRoot)) (Variables|Default|GetButtonInitialLocation) DeltaSeconds 1e+01) false false))

(fn ConstructionScript)

(fn IsInteractiveComponent
  (params (Interactor :type BPC%20Toolkit%20Motion%20Interactor%20Object%20Reference) (Component :type Primitive%20Component%20Object%20Reference))
  (return (== Component (Variables|Default|GetButton))))

(fn OnComponentHovered
  (params (Interactor :type BPC%20Toolkit%20Motion%20Interactor%20Object%20Reference) (HoveredComponent :type Primitive%20Component%20Object%20Reference))
  (return false))

(fn OnComponentUnhovered
  (params (Interactor :type BPC%20Toolkit%20Motion%20Interactor%20Object%20Reference) (UnhoveredComponent :type Primitive%20Component%20Object%20Reference))
  (return false))

(fn OnDragCanceled
  (params (Interactor :type BPC%20Toolkit%20Motion%20Interactor%20Object%20Reference))
  (return false))

(fn OnDragDetected
  (params (Interactor :type BPC%20Toolkit%20Motion%20Interactor%20Object%20Reference))
  (return false))

(fn OnDragMove
  (params (Interactor :type BPC%20Toolkit%20Motion%20Interactor%20Object%20Reference))
  (return false))

(fn OnGrabPressed
  (params (Interactor :type BPC%20Toolkit%20Motion%20Interactor%20Object%20Reference))
  (CallFunction|ButtonPressed)
  (return false))

(fn OnGrabReleased
  (params (Interactor :type BPC%20Toolkit%20Motion%20Interactor%20Object%20Reference))
  (return false))

(fn OnHoverEnter
  (params (Interactor :type BPC%20Toolkit%20Motion%20Interactor%20Object%20Reference))
  ;[1 1 1] 手柄震动
  (Class|PlayerController|PlayHapticEffect (Game|GetPlayerController 0) "/Game/PointVRToolkit/Blueprints/Characters/VirtualReality/VRHandHaptics.VRHandHaptics" (Default|GetHand Interactor) 0.2 false)
  ;[1 1 1] 记录手指首次接触到按钮时的位置
  (Variables|Default|SetInitialOverlapLocation (Transformation|GetWorldLocation (Default|GetOverlapShape Interactor)))
  (Rendering|Material|SetScalarParameterValueonMaterials (Variables|Default|GetButton) "PowerIntensity" 1.5)
  (return false))

(fn OnHoverLeave
  (params (Interactor :type BPC%20Toolkit%20Motion%20Interactor%20Object%20Reference))
  (bind _returnvalue (Rendering|Material|CreateDynamicMaterialInstance (Variables|Default|GetButton) 0 "/Game/ExtraTools/Materials/MI_KeyboardButton.MI_KeyboardButton" "None" :!class /Script/Engine.PrimitiveComponent))
  (Rendering|Material|SetScalarParameterValue _returnvalue "PowerIntensity" 1.0 :!class /Script/Engine.MaterialInstanceDynamic)
  (return false))

(fn OnHoverMove
  (params (Interactor :type BPC%20Toolkit%20Motion%20Interactor%20Object%20Reference))
  (bind _buttonroot (Variables|Default|GetButtonRoot))
  (bind _returnvalue (Transformation|GetWorldTransform _buttonroot))
  (bind _asbp_toolkit_vrhand (Utilities|Casting|CastToBP_ToolkitVRHand (Components|GetOwner Interactor)))
  (if (not (Variables|/Game/PointVRToolkit/Blueprints/Characters/VirtualReality/BP_ToolkitVRHand.BP_ToolkitVRHand_C|GetbIsLaserActivated _asbp_toolkit_vrhand))
    (bind _output_get (Variables|Default|SetPressDepth (Math|Float|Clamp(Float) (.z (- (Math|Transform|InverseTransformLocation _returnvalue (Variables|Default|GetInitialOverlapLocation)) (Math|Transform|InverseTransformLocation _returnvalue (Transformation|GetWorldLocation (Default|GetOverlapShape Interactor))))) 0.0 (Variables|Default|GetMaxPressDepth))))
    (Transformation|SetRelativeLocation (Variables|Default|GetButtonRoot) (- (Variables|Default|GetButtonInitialLocation) (Math|Vector|MakeVector 0.0 0.0 _output_get)) false false)
    (CallFunction|CheckReachedEnd)
    (return false)))

(fn OnUsePressed
  (params (Interactor :type BPC%20Toolkit%20Motion%20Interactor%20Object%20Reference))
  (return false))

(fn OnUseReleased
  (params (Interactor :type BPC%20Toolkit%20Motion%20Interactor%20Object%20Reference))
  (return false))
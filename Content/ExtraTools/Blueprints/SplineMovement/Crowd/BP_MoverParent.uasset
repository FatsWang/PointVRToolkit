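; BP_MoverParent is a parent actor that moves along a referenced spline path, looping from end to start.
; Each tick it advances its distance along the spline by axis, speed and delta time, then snaps location and rotation to that point with a height offset.
; A reversed path turns the yaw 180 degrees.
; Near the destination distance, it resets to the spline's start point and calls ReachedTheEnd.
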(event EventTick
  (params (DeltaSeconds :type Float%20%28single-precision%29))
  (CallFunction|AddMovement)
  (CallFunction|UpdateLocationandLocation)
  (if (Math|Float|NearlyEqual(Float) (Variables|Default|GetDestination) (Variables|Default|GetDistanceAlongSpline) 5.0)
    (CallFunction|ArrivedDestination)
    (Default|CallReachedtheEnd)))

(fn ConstructionScript)

(fn AddMovement
  (Variables|Default|SetDistanceAlongSpline (+ (* (Variables|Default|GetAxis) (Variables|Default|GetMoveSpeed) (Utilities|Time|GetWorldDeltaSeconds)) (Variables|Default|GetDistanceAlongSpline))))

(fn UpdateLocationandLocation
  (bind _actorheight (Variables|Default|GetActorHeight))
  (bind _distancealongspline (Variables|Default|GetDistanceAlongSpline))
  (bind _splineref (Variables|Default|GetSplineRef))
  (bind _distancealongspline_2 (Variables|Default|GetDistanceAlongSpline))
  (bind _spline (Variables|/Game/ExtraTools/Blueprints/SplineMovement/Crowd/BP_SplinePath.BP_SplinePath_C|GetSpline _splineref))
  (bind _returnvalue (Spline|GetLocationatDistanceAlongSpline _spline _distancealongspline_2 "World"))
  (bind _returnvalue_2 (Spline|GetRotationatDistanceAlongSpline _spline _distancealongspline "World"))
  (bind (_roll _pitch _yaw) (Math|Rotator|BreakRotator _returnvalue_2))
  (bind _returnvalue_3 (+ _returnvalue _actorheight))
  (if (Variables|/Game/ExtraTools/Blueprints/SplineMovement/Crowd/BP_SplinePath.BP_SplinePath_C|GetPathReverse _splineref)
    (Transformation|SetActorLocationAndRotation _returnvalue_3 (Math|Rotator|MakeRotator _roll _pitch (+ _yaw 1.8e+02)))
    (else
      (Transformation|SetActorLocationAndRotation _returnvalue_3 _returnvalue_2))))

(fn ArrivedDestination
  (Variables|Default|SetDistanceAlongSpline (Variables|/Game/ExtraTools/Blueprints/SplineMovement/Crowd/BP_SplinePath.BP_SplinePath_C|GetStartPoint (Variables|Default|GetSplineRef))))
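; BP_SplinePath is a crowd path that spawns a set number of randomly chosen actor classes to travel along its spline.
; Spawning runs on BeginPlay when StartAtBegining is set, or through the ActorStartMove event.
; Each actor receives an evenly spaced start distance, move speed, spline owner reference, and a destination and direction set by PathReverse.
; The path only initializes them; movement is left to the spawned actors.
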(event Custom|ActorStartMove
  (bind _amount (Variables|MoverConfig|GetAmount))
  (bind _actorclass (Variables|MoverConfig|GetActorClass))
  (bind _spline (Variables|Default|GetSpline))
  (bind _returnvalue (Spline|GetSplineLength _spline))
  (if (Variables|PathConfit|GetPathReverse)
    (Variables|Default|SetStartPoint _returnvalue)
    (Variables|Default|SetEndPoint 0.0)
    (Variables|Default|SetDirection -1.0)
    (else
      (Variables|Default|SetStartPoint 0.0)
      (Variables|Default|SetEndPoint _returnvalue)
      (Variables|Default|SetDirection 1.0)))
  (for _index (range 0 (- _amount 1))
    (Game|SpawnActorfromClass (Utilities|Array|Get(acopy) _actorclass (Math|Random|RandomInteger (Utilities|Array|Length _actorclass))) (Math|Transform|MakeTransform "0, 0, 0" "0, 0, 0" "1,1,1") "AlwaysSpawn" 0 (* _index (/ _returnvalue (Math|Conversions|ToFloat(Integer) _amount))) (Variables|Default|GetEndPoint) (Variables|Default|GetDirection) (Variables|MoverConfig|GetMoveSpeed) self 0)))

(event EventBeginPlay
  (if (Variables|PathConfit|GetStartAtBegining)
    (CallFunction|ActorStartMove)))

(fn ConstructionScript)
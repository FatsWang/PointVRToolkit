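; BP_SimplePickup is a VR interactive static mesh actor that interactors can grab, carry and drop.
; Grab input works as hold or toggle, and a grab by another interactor first releases the current one.
; Pickup locks the interactor's hover, disables physics and attaches to its GrabSocket, optionally snapping; dropping detaches and restores configured physics.
; Hovering toggles custom depth for highlighting, while drag and use callbacks are unhandled.
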(event Custom|OnPickedUp
  (params (Interactor :type BPC%20Toolkit%20Motion%20Interactor%20Object%20Reference))
  (bind _bsnaptopickuplocation (Variables|Pickup|GetbSnapToPickupLocation))
  (bind _returnvalue (select _bsnaptopickuplocation "SnapToTarget" "KeepWorld"))
  (bind _output_get (Variables|Default|SetCurrentInteractor Interactor))
  (Default|LockHovered _output_get)
  (Variables|Pickup|SetbIsPickedUp true)
  (if (Physics|IsSimulatingPhysics (Variables|Debug|GetStaticMeshComponent) "None")
    (Physics|SetSimulatePhysics (Variables|Debug|GetStaticMeshComponent) false))
  (Transformation|AttachComponentToComponent (Default|GetHoverShape (Variables|Default|GetCurrentInteractor)) "GrabSocket" _returnvalue _returnvalue "KeepWorld" true))

(event Custom|OnDropped
  (Default|UnlockHovered (Variables|Default|GetCurrentInteractor))
  (Variables|Pickup|SetbIsPickedUp false)
  (Transformation|DetachFromActor "KeepWorld" "KeepWorld" "KeepWorld")
  (Physics|SetSimulatePhysics (Variables|Debug|GetStaticMeshComponent) (Variables|Pickup|GetbSimPhysics)))

(fn ConstructionScript
  (Physics|SetSimulatePhysics (Variables|Debug|GetStaticMeshComponent) (Variables|Pickup|GetbSimPhysics)))

(fn IsInteractiveComponent
  (params (Interactor :type BPC%20Toolkit%20Motion%20Interactor%20Object%20Reference) (Component :type Primitive%20Component%20Object%20Reference))
  (return (== Component (Variables|Debug|GetStaticMeshComponent))))

(fn OnComponentHovered
  (params (Interactor :type BPC%20Toolkit%20Motion%20Interactor%20Object%20Reference) (HoveredComponent :type Primitive%20Component%20Object%20Reference))
  (return false))

(fn OnComponentUnhovered
  (params (Interactor :type BPC%20Toolkit%20Motion%20Interactor%20Object%20Reference) (UnhoveredComponent :type Primitive%20Component%20Object%20Reference))
  (return false))

(fn OnDragCanceled
  (params (Interactor :type BPC%20Toolkit%20Motion%20Interactor%20Object%20Reference))
  (return false))

(fn OnDragDetected
  (params (Interactor :type BPC%20Toolkit%20Motion%20Interactor%20Object%20Reference))
  (return false))

(fn OnDragMove
  (params (Interactor :type BPC%20Toolkit%20Motion%20Interactor%20Object%20Reference))
  (return false))

(fn OnGrabPressed
  (params (Interactor :type BPC%20Toolkit%20Motion%20Interactor%20Object%20Reference))
  (bind _currentinteractor (Variables|Default|GetCurrentInteractor))
  (if (and (!= Interactor _currentinteractor) (Utilities|IsValid _currentinteractor))
    (CallFunction|OnDropped))
  (if (Variables|Pickup|GetbShouldHoldToPickup)
    (CallFunction|OnPickedUp Interactor)
    (elif (Variables|Pickup|GetbIsPickedUp)
      (CallFunction|OnDropped)
      (else
        (CallFunction|OnPickedUp Interactor))))
  (return true))

(fn OnGrabReleased
  (params (Interactor :type BPC%20Toolkit%20Motion%20Interactor%20Object%20Reference))
  (if (== Interactor (Variables|Default|GetCurrentInteractor))
    (if (Variables|Pickup|GetbShouldHoldToPickup)
      (CallFunction|OnDropped)))
  (return false))

(fn OnHoverEnter
  (params (Interactor :type BPC%20Toolkit%20Motion%20Interactor%20Object%20Reference))
  (Rendering|SetRenderCustomDepth (Variables|Debug|GetStaticMeshComponent) true)
  (return false))

(fn OnHoverLeave
  (params (Interactor :type BPC%20Toolkit%20Motion%20Interactor%20Object%20Reference))
  (Rendering|SetRenderCustomDepth (Variables|Debug|GetStaticMeshComponent) false)
  (return false))

(fn OnHoverMove
  (params (Interactor :type BPC%20Toolkit%20Motion%20Interactor%20Object%20Reference))
  (return false))

(fn OnUsePressed
  (params (Interactor :type BPC%20Toolkit%20Motion%20Interactor%20Object%20Reference))
  (return false))

(fn OnUseReleased
  (params (Interactor :type BPC%20Toolkit%20Motion%20Interactor%20Object%20Reference))
  (return false))
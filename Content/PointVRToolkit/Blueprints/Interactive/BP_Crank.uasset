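; BP_Crank is a VR interactive crank that a hand drags around one axis, clamped between minimum and maximum turn counts.
; While dragging, it converts the hand's actor-local movement into an arcball angle delta that accumulates into the roll of RotateRoot.
; On drag cancel, optional fake inertia enables Tick to decay the last delta, then disables Tick near zero.
; Hover toggles custom depth, and a debug flag shows arrows and turn-count text.
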(event EventTick
  (params (DeltaSeconds :type Float%20%28single-precision%29))
  ;[1 1 0] 这里让曲柄在旋转结束后模拟一段减速旋转的惯性效果
  (bind _output_get (Variables|Crank|SetCurrentDeltaAngle (Math|Interpolation|FInterptoConstant (Variables|Crank|GetCurrentDeltaAngle) 0.0 DeltaSeconds (Variables|Crank|GetDeltaAngleInterpSpeed))))
  (bind _output_get_2 (Variables|Crank|SetCurrentDegree (Math|Float|Clamp(Float) (+ _output_get (Variables|Crank|GetCurrentDegree)) (* (Variables|Crank|GetMinTurns) 3.6e+02) (* (Variables|Crank|GetMaxTurns) 3.6e+02))))
  (Transformation|SetRelativeRotation (Variables|Default|GetRotateRoot) (Math|Rotator|MakeRotator _output_get_2 0.0 0.0) false false)
  (if (Math|Float|NearlyEqual(Float) (Variables|Crank|GetCurrentDeltaAngle) 0.0 1e-06)
    (Actor|Tick|SetActorTickEnabled false) ; 这里保证Tick在不需要的时候不会执行
  )
  ;[1 1 0] 用于Debug用的，最后发布阶段可以删除
  (if (Variables|DebugSettings|GetbShowDebug)
    (Rendering|Components|TextRender|SetText (Variables|Default|GetDebugText) (|SetDebugText_2_2))))

(fn ConstructionScript
  (bind _debugtext (Variables|Default|GetDebugText))
  (Development|SetHiddeninGame (Variables|Default|GetRightArrow) (not (Variables|DebugSettings|GetbShowDebug)) false)
  (if (not (Variables|/Script/Engine.SceneComponent|GetbHiddenInGame _debugtext))
    (Rendering|Components|TextRender|SetText _debugtext (Utilities|Text|MakeLiteralText "Turns:  "))))

(fn IsInteractiveComponent
  (params (Interactor :type BPC%20Toolkit%20Motion%20Interactor%20Object%20Reference) (Component :type Primitive%20Component%20Object%20Reference))
  (return (== Component (Variables|Default|GetCrank))))

(fn OnComponentHovered
  (params (Interactor :type BPC%20Toolkit%20Motion%20Interactor%20Object%20Reference) (HoveredComponent :type Primitive%20Component%20Object%20Reference))
  (return false))

(fn OnComponentUnhovered
  (params (Interactor :type BPC%20Toolkit%20Motion%20Interactor%20Object%20Reference) (UnhoveredComponent :type Primitive%20Component%20Object%20Reference))
  (return false))

(fn OnDragCanceled
  (params (Interactor :type BPC%20Toolkit%20Motion%20Interactor%20Object%20Reference))
  (Default|UnlockHovered Interactor)
  (if (Variables|Crank|GetbSimulateInertia)
    (Actor|Tick|SetActorTickEnabled true)
    (return false)))

(fn OnDragDetected
  (params (Interactor :type BPC%20Toolkit%20Motion%20Interactor%20Object%20Reference))
  (Default|LockHovered Interactor)
  (bind _output_get (Variables|Crank|SetCurrentFrameHandPosition (Math|Transform|InverseTransformLocation (Transformation|GetActorTransform) (Transformation|GetWorldLocation (Default|GetHoverShape Interactor)))))
  (Variables|Crank|SetPreviousFrameHandPosition _output_get)
  (return true))

(fn OnDragMove
  (params (Interactor :type BPC%20Toolkit%20Motion%20Interactor%20Object%20Reference))
  (Variables|Crank|SetCurrentFrameHandPosition (Math|Transform|InverseTransformLocation (Transformation|GetActorTransform) (Transformation|GetWorldLocation (Default|GetHoverShape Interactor)))) ; 当前帧的手部位置（相对）
  (bind _output_get (Variables|Crank|SetCurrentDeltaAngle (CallFunction|CalculateArcballAngleAroundAxis "NewEnumerator0" (Variables|Crank|GetPreviousFrameHandPosition) (Variables|Crank|GetCurrentFrameHandPosition))))
  (bind _output_get_2 (Variables|Crank|SetCurrentDegree (Math|Float|Clamp(Float) (+ _output_get (Variables|Crank|GetCurrentDegree)) (* (Variables|Crank|GetMinTurns) 3.6e+02) (* (Variables|Crank|GetMaxTurns) 3.6e+02))))
  (Transformation|SetRelativeRotation (Variables|Default|GetRotateRoot) (Math|Rotator|MakeRotator _output_get_2 0.0 0.0) false false)
  (Variables|Crank|SetPreviousFrameHandPosition (Variables|Crank|GetCurrentFrameHandPosition)) ; 当前帧的手部位置将作为下一帧的上一帧位置
  (if (Variables|DebugSettings|GetbShowDebug)
    ;[1 1 0] 用于Debug用的，最后发布阶段可以删除
    (Rendering|Components|TextRender|SetText (Variables|Default|GetDebugText) (|SetDebugText)))
  (return false))

(fn OnGrabPressed
  (params (Interactor :type BPC%20Toolkit%20Motion%20Interactor%20Object%20Reference))
  (return false))

(fn OnGrabReleased
  (params (Interactor :type BPC%20Toolkit%20Motion%20Interactor%20Object%20Reference))
  (return false))

(fn OnHoverEnter
  (params (Interactor :type BPC%20Toolkit%20Motion%20Interactor%20Object%20Reference))
  (Rendering|SetRenderCustomDepth (Variables|Default|GetCrank) true)
  (return false))

(fn OnHoverLeave
  (params (Interactor :type BPC%20Toolkit%20Motion%20Interactor%20Object%20Reference))
  (Rendering|SetRenderCustomDepth (Variables|Default|GetCrank) false)
  (return false))

(fn OnHoverMove
  (params (Interactor :type BPC%20Toolkit%20Motion%20Interactor%20Object%20Reference))
  (return false))

(fn OnUsePressed
  (params (Interactor :type BPC%20Toolkit%20Motion%20Interactor%20Object%20Reference))
  (return false))

(fn OnUseReleased
  (params (Interactor :type BPC%20Toolkit%20Motion%20Interactor%20Object%20Reference))
  (return false))
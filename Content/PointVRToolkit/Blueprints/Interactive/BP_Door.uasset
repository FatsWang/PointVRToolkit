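; BP_Door is a VR interactive door that an interactor drags by its Box component to swing around a hinge.
; While dragged, the interactor's hover-shape position in door space becomes a yaw angle on RotateRoot, offset from the initial drag angle and clamped to MinAngle and MaxAngle.
; When the drag is canceled, Tick carries the last angle delta on as decaying momentum, then disables itself once it reaches zero.
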(event EventBeginPlay)

(event Collision|EventActorBeginOverlap
  (params (OtherActor :type Actor%20Object%20Reference)))

(event EventTick
  (params (DeltaSeconds :type Float%20%28single-precision%29))
  (bind _output_get (Variables|Default|SetDeltaAngle (Math|Interpolation|FInterptoConstant (Variables|Default|GetDeltaAngle) 0.0 DeltaSeconds 0.98)))
  (bind _output_get_2 (Variables|Default|SetCurrentAngle (Math|Float|Clamp(Float) (+ _output_get (Variables|Default|GetCurrentAngle)) (Variables|Default|GetMinAngle) (Variables|Default|GetMaxAngle))))
  (Transformation|SetRelativeRotation (Variables|Default|GetRotateRoot) (Math|Rotator|MakeRotator 0.0 0.0 _output_get_2) false false)
  (if (== (Variables|Default|GetDeltaAngle) 0.0)
    (Actor|Tick|SetActorTickEnabled false)))

(fn ConstructionScript)

(fn IsInteractiveComponent
  (params (Interactor :type BPC%20Toolkit%20Motion%20Interactor%20Object%20Reference) (Component :type Primitive%20Component%20Object%20Reference))
  (return (== Component (Variables|Default|GetBox))))

(fn OnComponentHovered
  (params (Interactor :type BPC%20Toolkit%20Motion%20Interactor%20Object%20Reference) (HoveredComponent :type Primitive%20Component%20Object%20Reference))
  (return false))

(fn OnComponentUnhovered
  (params (Interactor :type BPC%20Toolkit%20Motion%20Interactor%20Object%20Reference) (UnhoveredComponent :type Primitive%20Component%20Object%20Reference))
  (return false))

(fn OnDragCanceled
  (params (Interactor :type BPC%20Toolkit%20Motion%20Interactor%20Object%20Reference))
  (Actor|Tick|SetActorTickEnabled true)
  (return false))

(fn OnDragDetected
  (params (Interactor :type BPC%20Toolkit%20Motion%20Interactor%20Object%20Reference))
  (Variables|Default|SetInitialDragOffset (- (CallFunction|CalculateRotationAngleAroundAxis "NewEnumerator2" (- (Math|Transform|InverseTransformLocation (Transformation|GetActorTransform) (Transformation|GetWorldLocation (Default|GetHoverShape Interactor))) (Variables|/Script/Engine.SceneComponent|GetRelativeLocation (Variables|Default|GetRotateRoot)))) (Variables|Default|GetCurrentAngle)))
  (return true))

(fn OnDragMove
  (params (Interactor :type BPC%20Toolkit%20Motion%20Interactor%20Object%20Reference))
  (bind _hovershape (Default|GetHoverShape Interactor))
  (bind _returnvalue (Transformation|GetActorTransform))
  (bind _rotateroot (Variables|Default|GetRotateRoot))
  (bind _maxangle (Variables|Default|GetMaxAngle))
  (bind _minangle (Variables|Default|GetMinAngle))
  (bind _initialdragoffset (Variables|Default|GetInitialDragOffset))
  (bind _returnvalue_2 (Transformation|GetWorldLocation _hovershape))
  (bind _relativelocation (Variables|/Script/Engine.SceneComponent|GetRelativeLocation _rotateroot))
  (bind _returnvalue_3 (Math|Transform|InverseTransformLocation _returnvalue _returnvalue_2))
  (bind _returnvalue_4 (- _returnvalue_3 _relativelocation))
  (bind _angle (CallFunction|CalculateRotationAngleAroundAxis "NewEnumerator2" _returnvalue_4))
  (bind _returnvalue_5 (- _angle _initialdragoffset))
  (bind _returnvalue_6 (Math|Float|Clamp(Float) _returnvalue_5 _minangle _maxangle))
  (Variables|Default|SetDeltaAngle (- _returnvalue_6 (Variables|Default|GetCurrentAngle)))
  (bind _output_get (Variables|Default|SetCurrentAngle _returnvalue_6))
  (Transformation|SetRelativeRotation (Variables|Default|GetRotateRoot) (Math|Rotator|MakeRotator 0.0 0.0 _output_get) false false)
  (return false))

(fn OnGrabPressed
  (params (Interactor :type BPC%20Toolkit%20Motion%20Interactor%20Object%20Reference))
  (return false))

(fn OnGrabReleased
  (params (Interactor :type BPC%20Toolkit%20Motion%20Interactor%20Object%20Reference))
  (return false))

(fn OnHoverEnter
  (params (Interactor :type BPC%20Toolkit%20Motion%20Interactor%20Object%20Reference))
  (return false))

(fn OnHoverLeave
  (params (Interactor :type BPC%20Toolkit%20Motion%20Interactor%20Object%20Reference))
  (return false))

(fn OnHoverMove
  (params (Interactor :type BPC%20Toolkit%20Motion%20Interactor%20Object%20Reference))
  (return false))

(fn OnUsePressed
  (params (Interactor :type BPC%20Toolkit%20Motion%20Interactor%20Object%20Reference))
  (return false))

(fn OnUseReleased
  (params (Interactor :type BPC%20Toolkit%20Motion%20Interactor%20Object%20Reference))
  (return false))
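; BP_TeleportTarget is a VR teleport point that moves the toolkit pawn to its exact location and facing.
; While an active teleport trace is on it, the hand rumbles and a timeline raises an arrow plane, yawed toward the camera.
; Releasing click fades the camera out, deactivates the hand's teleport, moves the pawn, fires OnTeleportToTarget, then fades back in.
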(event Custom|PlayArrowAnim
  (Rendering|SetVisibility (Variables|Default|GetPlane) true false)
  (bind _alpha (Timeline|ArrowAnimTimeline PlayFromStart)
    (:Update
      (Transformation|SetRelativeLocationAndRotation (Variables|Default|GetPlaneRoot) (Math|Vector|Lerp(Vector) "0, 0, 0" "0, 0,50.000000" _alpha) (Math|Rotator|MakeRotator 0.0 0.0 (.yaw (Math|Rotator|FindLookatRotation (Transformation|GetActorLocation) (Camera|GetCameraLocation (Game|GetPlayerCameraManager 0))))) false false))))

(event Custom|StopArrowAnim
  (Rendering|SetVisibility (Variables|Default|GetPlane) false false)
  (bind _alpha (Timeline|ArrowAnimTimeline Stop)
    (:Update
      (Transformation|SetRelativeLocationAndRotation (Variables|Default|GetPlaneRoot) (Math|Vector|Lerp(Vector) "0, 0, 0" "0, 0,50.000000" _alpha) (Math|Rotator|MakeRotator 0.0 0.0 (.yaw (Math|Rotator|FindLookatRotation (Transformation|GetActorLocation) (Camera|GetCameraLocation (Game|GetPlayerCameraManager 0))))) false false))))

(event Custom|EventTeleportPlayer
  (params (Hand :type BP%20Toolkit%20VR%20Hand%20Object%20Reference))
  ;[1 1 0] 传送到该TeleportTarget的位置并且固定朝向为TeleportTarget的X方向
  (bind _asbp_toolkit_vrpawn (Utilities|Casting|CastToBP_ToolkitVRPawn (Components|GetOwner Hand)))
  (Variables|/Game/PointVRToolkit/Blueprints/Player/VirtualReality/BP_ToolkitVRPawn.BP_ToolkitVRPawn_C|SetbIsTeleporting _asbp_toolkit_vrpawn true)
  (CameraFades|StartCameraFade :self (Game|GetPlayerCameraManager 0) :ToAlpha 1.0 :Duration (Variables|/Game/PointVRToolkit/Blueprints/Player/VirtualReality/BP_ToolkitVRPawn.BP_ToolkitVRPawn_C|GetFadeOutDuration _asbp_toolkit_vrpawn) :bHoldWhenFinished true)
  (Utilities|FlowControl|Delay (Variables|/Game/PointVRToolkit/Blueprints/Player/VirtualReality/BP_ToolkitVRPawn.BP_ToolkitVRPawn_C|GetFadeOutDuration _asbp_toolkit_vrpawn))
  (Default|DeactivateTeleport Hand)
  (Transformation|SetActorLocationAndRotation _asbp_toolkit_vrpawn (Transformation|GetActorLocation) (Math|Rotator|MakeRotator 0.0 0.0 (.yaw (Transformation|GetActorRotation))) false true)
  (Default|CallOnTeleporttoTarget) ; 传送到该位置之后调用该调度器
  (CameraFades|StartCameraFade :self (Game|GetPlayerCameraManager 0) :FromAlpha 1.0 :Duration (Variables|/Game/PointVRToolkit/Blueprints/Player/VirtualReality/BP_ToolkitVRPawn.BP_ToolkitVRPawn_C|GetFadeOutDuration _asbp_toolkit_vrpawn))
  (Variables|/Game/PointVRToolkit/Blueprints/Player/VirtualReality/BP_ToolkitVRPawn.BP_ToolkitVRPawn_C|SetbIsTeleporting _asbp_toolkit_vrpawn false))

(event EventBeginPlay
  (Rendering|SetVisibility (Variables|Default|GetPlane) false false))

(fn ConstructionScript)

(fn OnClickPressed
  (params (Interactor :type BPC%20Toolkit%20Trace%20Interactor%20Object%20Reference) (TraceHit :type Hit%20Result%20Structure%20%28by%20ref%29))
  (return false))

(fn OnClickReleased
  (params (Interactor :type BPC%20Toolkit%20Trace%20Interactor%20Object%20Reference) (TraceHit :type Hit%20Result%20Structure%20%28by%20ref%29))
  (bind _asbp_toolkit_vrhand (Utilities|Casting|CastToBP_ToolkitVRHand (Components|GetOwner Interactor)))
  (if (Variables|/Game/PointVRToolkit/Blueprints/Player/VirtualReality/BP_ToolkitVRHand.BP_ToolkitVRHand_C|GetbIsTeleportActivated _asbp_toolkit_vrhand)
    (CallFunction|EventTeleportPlayer _asbp_toolkit_vrhand)
    (return false)))

(fn OnComponentHovered
  (params (Interactor :type BPC%20Toolkit%20Trace%20Interactor%20Object%20Reference) (TraceHit :type Hit%20Result%20Structure%20%28by%20ref%29) (CurrentComponent :type Primitive%20Component%20Object%20Reference))
  (return false))

(fn OnComponentUnhovered
  (params (Interactor :type BPC%20Toolkit%20Trace%20Interactor%20Object%20Reference) (TraceHit :type Hit%20Result%20Structure%20%28by%20ref%29) (PreviousComponent :type Primitive%20Component%20Object%20Reference))
  (return false))

(fn OnDragCanceled
  (params (Interactor :type BPC%20Toolkit%20Trace%20Interactor%20Object%20Reference) (TraceHit :type Hit%20Result%20Structure%20%28by%20ref%29))
  (return false))

(fn OnDragDetected
  (params (Interactor :type BPC%20Toolkit%20Trace%20Interactor%20Object%20Reference) (TraceHit :type Hit%20Result%20Structure%20%28by%20ref%29))
  (return false))

(fn OnDragMove
  (params (Interactor :type BPC%20Toolkit%20Trace%20Interactor%20Object%20Reference) (TraceHit :type Hit%20Result%20Structure%20%28by%20ref%29))
  (return false))

(fn OnTraceEnter
  (params (Interactor :type BPC%20Toolkit%20Trace%20Interactor%20Object%20Reference) (TraceHit :type Hit%20Result%20Structure%20%28by%20ref%29))
  (bind _asbp_toolkit_vrhand (Utilities|Casting|CastToBP_ToolkitVRHand (Components|GetOwner Interactor)))
  (if (Variables|/Game/PointVRToolkit/Blueprints/Player/VirtualReality/BP_ToolkitVRHand.BP_ToolkitVRHand_C|GetbIsTeleportActivated _asbp_toolkit_vrhand)
    (Default|RumbleHand _asbp_toolkit_vrhand 0 0.5)
    (CallFunction|PlayArrowAnim)
    (return false)))

(fn OnTraceLeave
  (params (Interactor :type BPC%20Toolkit%20Trace%20Interactor%20Object%20Reference) (TraceHit :type Hit%20Result%20Structure%20%28by%20ref%29))
  (CallFunction|StopArrowAnim)
  (return false))

(fn OnTraceMove
  (params (Interactor :type BPC%20Toolkit%20Trace%20Interactor%20Object%20Reference) (TraceHit :type Hit%20Result%20Structure%20%28by%20ref%29))
  (return false))
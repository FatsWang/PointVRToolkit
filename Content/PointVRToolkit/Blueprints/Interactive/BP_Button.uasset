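; VR push button that an interactor presses physically, firing OnButtonPressed when fully depressed.
; Hover enter stores the contact point and enables custom depth highlighting; hover move converts finger travel into clamped local-Z depth that offsets ButtonRoot.
; A DoOnce limits the event to one firing until hover movement registers a shallower depth.
; Hover leave clears the highlight and enables Tick, which eases the button back to rest, then disables itself.
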(event Custom|CheckButtonPressed
  (if (>= (Variables|Default|GetButtonPressAmount) (Variables|Default|GetMaxButtonPress))
    (Utilities|FlowControl|DoOnce false :!label _label
      (:Completed
        ;[1 1 0] 这个事件调度器以后可以设置签名发送数据
        (Default|CallOnButtonPressed)))
    (else
      (goto _label Reset))))

(event EventTick
  (params (DeltaSeconds :type Float%20%28single-precision%29))
  (Transformation|SetRelativeLocation (Variables|Default|GetButtonRoot) (Math|Interpolation|VInterpTo (Variables|/Script/Engine.SceneComponent|GetRelativeLocation (Variables|Default|GetButtonRoot)) (Variables|Default|GetButtonInitialLocation) DeltaSeconds 1e+01) false false)
  (if (Math|Vector|Equal(Vector) (Variables|/Script/Engine.SceneComponent|GetRelativeLocation (Variables|Default|GetButtonRoot)) (Variables|Default|GetButtonInitialLocation) 0.0001)
    (Actor|Tick|SetActorTickEnabled false)))

(event EventBeginPlay
  (Variables|Default|SetButtonInitialLocation (Variables|/Script/Engine.SceneComponent|GetRelativeLocation (Variables|Default|GetButtonRoot))))

(fn ConstructionScript)

(fn IsInteractiveComponent
  (params (Interactor :type BPC%20Toolkit%20Motion%20Interactor%20Object%20Reference) (Component :type Primitive%20Component%20Object%20Reference))
  (return (== Component (Variables|Default|GetButton))))

(fn OnComponentHovered
  (params (Interactor :type BPC%20Toolkit%20Motion%20Interactor%20Object%20Reference) (HoveredComponent :type Primitive%20Component%20Object%20Reference))
  (return false))

(fn OnComponentUnhovered
  (params (Interactor :type BPC%20Toolkit%20Motion%20Interactor%20Object%20Reference) (UnhoveredComponent :type Primitive%20Component%20Object%20Reference))
  (return false))

(fn OnDragCanceled
  (params (Interactor :type BPC%20Toolkit%20Motion%20Interactor%20Object%20Reference))
  (return false))

(fn OnDragDetected
  (params (Interactor :type BPC%20Toolkit%20Motion%20Interactor%20Object%20Reference))
  (return false))

(fn OnDragMove
  (params (Interactor :type BPC%20Toolkit%20Motion%20Interactor%20Object%20Reference))
  (return false))

(fn OnGrabPressed
  (params (Interactor :type BPC%20Toolkit%20Motion%20Interactor%20Object%20Reference))
  (return false))

(fn OnGrabReleased
  (params (Interactor :type BPC%20Toolkit%20Motion%20Interactor%20Object%20Reference))
  (return false))

(fn OnHoverEnter
  (params (Interactor :type BPC%20Toolkit%20Motion%20Interactor%20Object%20Reference))
  (Variables|Default|SetInitialOverlapLocation (Transformation|GetWorldLocation (Default|GetHoverShape Interactor)))
  (Rendering|SetRenderCustomDepth (Variables|Default|GetButton) true)
  (return false))

(fn OnHoverLeave
  (params (Interactor :type BPC%20Toolkit%20Motion%20Interactor%20Object%20Reference))
  (Rendering|SetRenderCustomDepth (Variables|Default|GetButton) false)
  (Actor|Tick|SetActorTickEnabled true)
  (return false))

(fn OnHoverMove
  (params (Interactor :type BPC%20Toolkit%20Motion%20Interactor%20Object%20Reference))
  (bind _buttonroot (Variables|Default|GetButtonRoot))
  (bind _returnvalue (Transformation|GetWorldTransform _buttonroot))
  (bind _output_get (Variables|Default|SetButtonPressAmount (Math|Float|Clamp(Float) (.z (- (Math|Transform|InverseTransformLocation _returnvalue (Variables|Default|GetInitialOverlapLocation)) (Math|Transform|InverseTransformLocation _returnvalue (Transformation|GetWorldLocation (Default|GetHoverShape Interactor))))) 0.0 (Variables|Default|GetMaxButtonPress))))
  (Transformation|SetRelativeLocation (Variables|Default|GetButtonRoot) (- (Variables|Default|GetButtonInitialLocation) (Math|Vector|MakeVector 0.0 0.0 _output_get)) false false)
  (CallFunction|CheckButtonPressed)
  (return false))

(fn OnUsePressed
  (params (Interactor :type BPC%20Toolkit%20Motion%20Interactor%20Object%20Reference))
  (return false))

(fn OnUseReleased
  (params (Interactor :type BPC%20Toolkit%20Motion%20Interactor%20Object%20Reference))
  (return false))
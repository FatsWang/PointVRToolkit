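; VR lever actor that an interactor drags by its handle to rotate between a minimum and maximum angle.
; Drag start stores an angular offset; each move projects the interactor's local position into an angle, clamps it and sets RotateRoot's roll.
; A DoOnce multi-input gate, reset between limits, fires max or min reached events, logic the author flags as rough.
; Hovering highlights the handle through custom depth.
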(event Custom|CheckLeverRotation
  ;[1 1 0] 这部分逻辑处理的不太好，本意是想让控制杆达到最大值或最小值时能够发出信号
  (if (Math|Float|InRange(Float) (Variables|Lever|GetCurrentAngle) (Variables|Lever|GetMinAngle) (Variables|Lever|GetMaxAngle) false false)
    (goto _label Reset%20In)
    (elif (== (Variables|Lever|GetCurrentAngle) (Variables|Lever|GetMaxAngle))
      (|DoOnceMultiInput :!label _label
        (:A%20Out
          (Default|CallOnReachMaxDegree))
        (:B%20Out
          (Default|CallOnReachMinDegree)))
      (else
        (goto _label B%20In)))))

(event EventBeginPlay)

(event Collision|EventActorBeginOverlap
  (params (OtherActor :type Actor%20Object%20Reference)))

(fn ConstructionScript)

(fn IsInteractiveComponent
  (params (Interactor :type BPC%20Toolkit%20Motion%20Interactor%20Object%20Reference) (Component :type Primitive%20Component%20Object%20Reference))
  (return (== Component (Variables|Default|GetLeverHandle))))

(fn OnComponentHovered
  (params (Interactor :type BPC%20Toolkit%20Motion%20Interactor%20Object%20Reference) (HoveredComponent :type Primitive%20Component%20Object%20Reference))
  (return false))

(fn OnComponentUnhovered
  (params (Interactor :type BPC%20Toolkit%20Motion%20Interactor%20Object%20Reference) (UnhoveredComponent :type Primitive%20Component%20Object%20Reference))
  (return false))

(fn OnDragCanceled
  (params (Interactor :type BPC%20Toolkit%20Motion%20Interactor%20Object%20Reference))
  (return false))

(fn OnDragDetected
  (params (Interactor :type BPC%20Toolkit%20Motion%20Interactor%20Object%20Reference))
  (Variables|Lever|SetInitialDragOffset (- (CallFunction|CalculateRotationAngleAroundAxis "NewEnumerator0" (- (Math|Transform|InverseTransformLocation (Transformation|GetActorTransform) (Transformation|GetWorldLocation (Default|GetHoverShape Interactor))) (Variables|/Script/Engine.SceneComponent|GetRelativeLocation (Variables|Default|GetRotateRoot)))) (Variables|Lever|GetCurrentAngle)))
  (return true))

(fn OnDragMove
  (params (Interactor :type BPC%20Toolkit%20Motion%20Interactor%20Object%20Reference))
  (bind _output_get (Variables|Lever|SetCurrentAngle (Math|Float|Clamp(Float) (- (CallFunction|CalculateRotationAngleAroundAxis "NewEnumerator0" (- (Math|Transform|InverseTransformLocation (Transformation|GetActorTransform) (Transformation|GetWorldLocation (Default|GetHoverShape Interactor))) (Variables|/Script/Engine.SceneComponent|GetRelativeLocation (Variables|Default|GetRotateRoot)))) (Variables|Lever|GetInitialDragOffset)) (Variables|Lever|GetMinAngle) (Variables|Lever|GetMaxAngle))))
  (Transformation|SetRelativeRotation (Variables|Default|GetRotateRoot) (Math|Rotator|MakeRotator _output_get 0.0 0.0) false false)
  (CallFunction|CheckLeverRotation)
  (return false))

(fn OnGrabPressed
  (params (Interactor :type BPC%20Toolkit%20Motion%20Interactor%20Object%20Reference))
  (return false))

(fn OnGrabReleased
  (params (Interactor :type BPC%20Toolkit%20Motion%20Interactor%20Object%20Reference))
  (return false))

(fn OnHoverEnter
  (params (Interactor :type BPC%20Toolkit%20Motion%20Interactor%20Object%20Reference))
  (Rendering|SetRenderCustomDepth (Variables|Default|GetLeverHandle) true)
  (return false))

(fn OnHoverLeave
  (params (Interactor :type BPC%20Toolkit%20Motion%20Interactor%20Object%20Reference))
  (Rendering|SetRenderCustomDepth (Variables|Default|GetLeverHandle) false)
  (return false))

(fn OnHoverMove
  (params (Interactor :type BPC%20Toolkit%20Motion%20Interactor%20Object%20Reference))
  (return false))

(fn OnUsePressed
  (params (Interactor :type BPC%20Toolkit%20Motion%20Interactor%20Object%20Reference))
  (return false))

(fn OnUseReleased
  (params (Interactor :type BPC%20Toolkit%20Motion%20Interactor%20Object%20Reference))
  (return false))
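; BP_Arrow is a VR toolkit arrow projectile that damages and sticks into what it hits.
; ShootArrow sets the movement component's velocity and gravity scale and starts a lifespan so stray arrows expire.
; On hit it pushes physics-simulating components with an impulse, applies speed-scaled damage, and attaches to the hit component's bone.
; It then nudges itself randomly along local X to embed and clears its lifespan so it persists.
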(event Collision|EventHit
  (params (MyComp :type Primitive%20Component%20Object%20Reference) (Other :type Actor%20Object%20Reference) (OtherComp :type Primitive%20Component%20Object%20Reference) (bSelfMoved :type Boolean) (HitLocation :type Vector :default "0, 0, 0") (HitNormal :type Vector :default "0, 0, 0") (NormalImpulse :type Vector :default "0, 0, 0") (Hit :type Hit%20Result%20Structure%20%28by%20ref%29))
  (bind _returnvalue (Transformation|GetComponentVelocity MyComp))
  (if (Physics|IsSimulatingPhysics OtherComp "None")
    (Utilities|FlowControl|Sequence
      (:then_0
        (Physics|AddImpulseatLocation OtherComp _returnvalue HitLocation "None")
        (Collision|IgnoreActorwhenMoving OtherComp self false))
      (:then_1
        (Game|Damage|ApplyDamage Other (* (Math|Vector|VectorLength _returnvalue) 0.05) 0 0 :!label _label)
        (Transformation|AttachComponentToComponent OtherComp (.HitBoneName (Collision|BreakHitResult Hit)) "KeepWorld" "KeepWorld" "KeepWorld" true)
        (Transformation|AddActorLocalOffset (Math|Vector|MakeVector (Math|Random|RandomFloatinRange 5.0 1e+01) 0.0 0.0) false true)
        (Actor|SetLifeSpan 0.0) ; 当箭射中某个对象时，就不销毁了
      ))
    (else
      (goto _label))))

(fn ConstructionScript)

(fn ShootArrow
  (params (GravityScale :type Float%20%28single-precision%29) (Velocity :type Vector))
  (bind _arrowmovement (Variables|Default|GetArrowMovement))
  (Variables|/Script/Engine.ProjectileMovementComponent|SetProjectileGravityScale _arrowmovement GravityScale)
  (Variables|/Script/Engine.MovementComponent|SetVelocity _arrowmovement Velocity)
  (Actor|SetLifeSpan 15.0) ; 大概箭射出去15秒就差不多可以销毁了
)
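; BP_Rotary is a VR interactive rotary switch that turns as an interactor drags it.
; Only the SMRotarySwitch component is interactive; hover, grab and use callbacks are unhandled.
; During a drag, the interactor's right vector in actor space is compared frame to frame with an arcball angle calculation around a fixed axis.
; The accumulated angle is clamped between MinAngle and MaxAngle and applied as roll on RotateRoot.
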(event EventBeginPlay)

(event Collision|EventActorBeginOverlap
  (params (OtherActor :type Actor%20Object%20Reference)))

(event EventTick
  (params (DeltaSeconds :type Float%20%28single-precision%29)))

(fn ConstructionScript)

(fn IsInteractiveComponent
  (params (Interactor :type BPC%20Toolkit%20Motion%20Interactor%20Object%20Reference) (Component :type Primitive%20Component%20Object%20Reference))
  (return (== Component (Variables|Default|GetSM_RotarySwitch))))

(fn OnComponentHovered
  (params (Interactor :type BPC%20Toolkit%20Motion%20Interactor%20Object%20Reference) (HoveredComponent :type Primitive%20Component%20Object%20Reference))
  (return false))

(fn OnComponentUnhovered
  (params (Interactor :type BPC%20Toolkit%20Motion%20Interactor%20Object%20Reference) (UnhoveredComponent :type Primitive%20Component%20Object%20Reference))
  (return false))

(fn OnDragCanceled
  (params (Interactor :type BPC%20Toolkit%20Motion%20Interactor%20Object%20Reference))
  (return false))

(fn OnDragDetected
  (params (Interactor :type BPC%20Toolkit%20Motion%20Interactor%20Object%20Reference))
  (bind _output_get (Variables|Default|SetCurrentFrameHandleDirection (Math|Transform|InverseTransformDirection (Transformation|GetActorTransform) (Math|Vector|GetRightVector Interactor))))
  (Variables|Default|SetPreviousFrameHandleDirection _output_get)
  (return true))

(fn OnDragMove
  (params (Interactor :type BPC%20Toolkit%20Motion%20Interactor%20Object%20Reference))
  (Variables|Default|SetCurrentFrameHandleDirection (Math|Transform|InverseTransformDirection (Transformation|GetActorTransform) (Math|Vector|GetRightVector Interactor)))
  (bind _output_get (Variables|Default|SetCurrentDeltaAngle (CallFunction|CalculateArcballAngleAroundAxis "NewEnumerator0" (Variables|Default|GetPreviousFrameHandleDirection) (Variables|Default|GetCurrentFrameHandleDirection))))
  (bind _output_get_2 (Variables|Default|SetCurrentAngle (Math|Float|Clamp(Float) (+ _output_get (Variables|Default|GetCurrentAngle)) (Variables|Default|GetMinAngle) (Variables|Default|GetMaxAngle))))
  (Transformation|SetRelativeRotation (Variables|Default|GetRotateRoot) (Math|Rotator|MakeRotator _output_get_2 0.0 0.0) false false)
  (Variables|Default|SetPreviousFrameHandleDirection (Variables|Default|GetCurrentFrameHandleDirection))
  (return false))

(fn OnGrabPressed
  (params (Interactor :type BPC%20Toolkit%20Motion%20Interactor%20Object%20Reference))
  (return false))

(fn OnGrabReleased
  (params (Interactor :type BPC%20Toolkit%20Motion%20Interactor%20Object%20Reference))
  (return false))

(fn OnHoverEnter
  (params (Interactor :type BPC%20Toolkit%20Motion%20Interactor%20Object%20Reference))
  (return false))

(fn OnHoverLeave
  (params (Interactor :type BPC%20Toolkit%20Motion%20Interactor%20Object%20Reference))
  (return false))

(fn OnHoverMove
  (params (Interactor :type BPC%20Toolkit%20Motion%20Interactor%20Object%20Reference))
  (return false))

(fn OnUsePressed
  (params (Interactor :type BPC%20Toolkit%20Motion%20Interactor%20Object%20Reference))
  (return false))

(fn OnUseReleased
  (params (Interactor :type BPC%20Toolkit%20Motion%20Interactor%20Object%20Reference))
  (return false))
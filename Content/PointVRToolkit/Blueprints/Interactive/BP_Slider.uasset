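; BP_Slider is a PointVR Toolkit interactive actor: a slider whose handle a VR interactor drags along one axis.
; Only SlideHandle counts as interactive, and hovering toggles its custom depth rendering, presumably for a highlight.
; Drag start stores the interactor's X offset in actor-local space; each move derives a SliderValue clamped between SlideMin and SlideMax and applies it to SlideRoot's relative location.
; Other interaction callbacks are unhandled stubs returning false.
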(event EventBeginPlay
  (bind _output_get (Variables|Slider|SetInitialSliderPosition (Variables|/Script/Engine.SceneComponent|GetRelativeLocation (Variables|Default|GetSlideRoot))))
  (Variables|Slider|SetSliderValue (.x _output_get)))

(event Collision|EventActorBeginOverlap
  (params (OtherActor :type Actor%20Object%20Reference)))

(event EventTick
  (params (DeltaSeconds :type Float%20%28single-precision%29)))

(fn ConstructionScript)

(fn IsInteractiveComponent
  (params (Interactor :type BPC%20Toolkit%20Motion%20Interactor%20Object%20Reference) (Component :type Primitive%20Component%20Object%20Reference))
  (return (== Component (Variables|Default|GetSlideHandle))))

(fn OnComponentHovered
  (params (Interactor :type BPC%20Toolkit%20Motion%20Interactor%20Object%20Reference) (HoveredComponent :type Primitive%20Component%20Object%20Reference))
  (return false))

(fn OnComponentUnhovered
  (params (Interactor :type BPC%20Toolkit%20Motion%20Interactor%20Object%20Reference) (UnhoveredComponent :type Primitive%20Component%20Object%20Reference))
  (return false))

(fn OnDragCanceled
  (params (Interactor :type BPC%20Toolkit%20Motion%20Interactor%20Object%20Reference))
  (return false))

(fn OnDragDetected
  (params (Interactor :type BPC%20Toolkit%20Motion%20Interactor%20Object%20Reference))
  (Variables|Slider|SetInitialDragOffset (- (.x (- (Math|Transform|InverseTransformLocation (Transformation|GetActorTransform) (Transformation|GetWorldLocation (Default|GetHoverShape Interactor))) (Variables|Slider|GetInitialSliderPosition))) (Variables|Slider|GetSliderValue)))
  (return true))

(fn OnDragMove
  (params (Interactor :type BPC%20Toolkit%20Motion%20Interactor%20Object%20Reference))
  (bind _output_get (Variables|Slider|SetSliderValue (Math|Float|Clamp(Float) (- (.x (- (Math|Transform|InverseTransformLocation (Transformation|GetActorTransform) (Transformation|GetWorldLocation (Default|GetHoverShape Interactor))) (Variables|Slider|GetInitialSliderPosition))) (Variables|Slider|GetInitialDragOffset)) (Variables|Slider|GetSlideMin) (Variables|Slider|GetSlideMax))))
  (Transformation|SetRelativeLocation (Variables|Default|GetSlideRoot) (Math|Vector|MakeVector _output_get 0.0 0.0) false false)
  (return false))

(fn OnGrabPressed
  (params (Interactor :type BPC%20Toolkit%20Motion%20Interactor%20Object%20Reference))
  (return false))

(fn OnGrabReleased
  (params (Interactor :type BPC%20Toolkit%20Motion%20Interactor%20Object%20Reference))
  (return false))

(fn OnHoverEnter
  (params (Interactor :type BPC%20Toolkit%20Motion%20Interactor%20Object%20Reference))
  (Rendering|SetRenderCustomDepth (Variables|Default|GetSlideHandle) true)
  (return false))

(fn OnHoverLeave
  (params (Interactor :type BPC%20Toolkit%20Motion%20Interactor%20Object%20Reference))
  (Rendering|SetRenderCustomDepth (Variables|Default|GetSlideHandle) false)
  (return false))

(fn OnHoverMove
  (params (Interactor :type BPC%20Toolkit%20Motion%20Interactor%20Object%20Reference))
  (return false))

(fn OnUsePressed
  (params (Interactor :type BPC%20Toolkit%20Motion%20Interactor%20Object%20Reference))
  (return false))

(fn OnUseReleased
  (params (Interactor :type BPC%20Toolkit%20Motion%20Interactor%20Object%20Reference))
  (return false))
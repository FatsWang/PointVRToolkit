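; Exploded-view tool that animates the actors attached to ExplodedRoot between saved collapsed and exploded layouts.
; The construction script gathers the actors, and setter events record their relative transforms for each layout.
; A timeline lerps those transforms forward to explode and in reverse to collapse, sampling current transforms as each animation starts.
; DoOnce gates make explode and collapse alternate, each re-armed when the timeline finishes.
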(event Custom|PlayExplodeAnimation
  (bind _outtransformarray (CallFunction|GetTransformArray))
  (Utilities|FlowControl|DoOnce false :!label _label
    (:Completed
      (Variables|Default|SetStartTransformArray _outtransformarray)
      (bind (_direction _alpha) (Timeline|ExplodeTimeline Play)
        (:Update
          (for (_array_element _array_index) (Variables|Default|GetExplodedActors)
            (Utilities|IsValid _array_element
              (:Is%20Valid
                (Transformation|SetActorRelativeTransform _array_element (Math|Transform|Lerp(Transform) (Utilities|Array|Get(acopy) (Variables|Default|GetStartTransformArray) _array_index) (Utilities|Array|Get(acopy) (Variables|Default|GetEndTransformArray) _array_index) _alpha) false false)))))
        (:Finished
          (switch Utilities|FlowControl|Switch|SwitchonETimelineDirection _direction
            (:Forward
              (Variables|Default|SetStartTransformArray (Variables|Default|GetCollapsedTransformArray))
              (Utilities|FlowControl|DoOnce true) ; enters at Reset
            )
            (:Backward
              (Variables|Default|SetEndTransformArray (Variables|Default|GetExplodedTransformArray))
              (goto _label Reset))))))))

(event Custom|SetCollapsedPosition
  (Variables|Default|SetCollapsedTransformArray (CallFunction|GetTransformArray)))

(event Custom|SetExplodedPosition
  (Variables|Default|SetExplodedTransformArray (CallFunction|GetTransformArray))
  (CallFunction|CollapsedView))

(event Custom|CollapsedView
  (CallFunction|ViewTransformArray (Variables|Default|GetCollapsedTransformArray)))

(event Custom|ExplodedView
  (CallFunction|ViewTransformArray (Variables|Default|GetExplodedTransformArray)))

(event Custom|ViewTransformArray
  (params (TransformArray :type Array%20of%20Transforms))
  (for (_array_element _array_index) (Variables|Default|GetExplodedActors)
    (Transformation|SetActorRelativeTransform _array_element (Utilities|Array|Get(acopy) TransformArray _array_index) false false)))

(event Custom|PlayCollapseAnimation
  (bind _outtransformarray (CallFunction|GetTransformArray))
  (Utilities|FlowControl|DoOnce true :!label _label
    (:Completed
      (Variables|Default|SetEndTransformArray _outtransformarray)
      (bind (_direction _alpha) (Timeline|ExplodeTimeline Reverse)
        (:Update
          (for (_array_element _array_index) (Variables|Default|GetExplodedActors)
            (Utilities|IsValid _array_element
              (:Is%20Valid
                (Transformation|SetActorRelativeTransform _array_element (Math|Transform|Lerp(Transform) (Utilities|Array|Get(acopy) (Variables|Default|GetStartTransformArray) _array_index) (Utilities|Array|Get(acopy) (Variables|Default|GetEndTransformArray) _array_index) _alpha) false false)))))
        (:Finished
          (switch Utilities|FlowControl|Switch|SwitchonETimelineDirection _direction
            (:Forward
              (Variables|Default|SetStartTransformArray (Variables|Default|GetCollapsedTransformArray))
              (goto _label Reset))
            (:Backward
              (Variables|Default|SetEndTransformArray (Variables|Default|GetExplodedTransformArray))
              (Utilities|FlowControl|DoOnce false) ; enters at Reset
            )))))))

(event EventBeginPlay
  (CallFunction|CollapsedView)
  (Variables|Default|SetStartTransformArray (Variables|Default|GetCollapsedTransformArray))
  (Variables|Default|SetEndTransformArray (Variables|Default|GetExplodedTransformArray)))

(fn ConstructionScript
  (bind _outattachedactors (CallFunction|GetAllAttachedActors (Variables|Default|GetExplodedRoot)))
  (Variables|Default|SetExplodedActors _outattachedactors))

(fn GetTransformArray
  (bind _temptransformarray (LocalVariables|GetTempTransformArray))
  (for _array_element (Variables|Default|GetExplodedActors)
    (Utilities|Array|Add _temptransformarray (Transformation|GetRelativeTransform (Variables|/Script/Engine.Actor|GetRootComponent _array_element))))
  (return _temptransformarray))
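; Editor placement tool actor that builds arrays of a chosen static mesh in its construction script.
; ArrayMode selects a 3D grid toward a handle point, rigid copies along a spline, or spline meshes deformed per point pair or per fixed-length segment.
; Spacing comes from SegmentSpaceBound, optionally reset to mesh bounds via a self-clearing toggle; spline modes measure along the forward axis, with Thickness scaling spline-mesh cross-sections.
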(fn ConstructionScript
  (bind _handlepoint (Variables|ArraySettings|GetHandlePoint))
  (bind _spline (Variables|Default|GetSpline))
  (bind _spline_2 (Variables|Default|GetSpline))
  (bind _thickness (Variables|ArraySettings|GetThickness))
  (bind _thickness_2 (Variables|ArraySettings|GetThickness))
  (bind _staticmesh (Variables|ArraySettings|GetStaticMesh))
  (bind _thickness_3 (Variables|ArraySettings|GetThickness))
  (bind _thickness_4 (Variables|ArraySettings|GetThickness))
  (bind _returnvalue (StaticMesh|GetBoundingBox _staticmesh))
  (Utilities|IsValid (Variables|ArraySettings|GetStaticMesh)
    (:Is%20Valid
      (if (Variables|ArraySettings|GetResetToMeshBound)
        (Variables|ArraySettings|SetSegmentSpaceBound (- (.max _returnvalue) (.min _returnvalue)))
        (Variables|ArraySettings|SetResetToMeshBound false))
      (LocalVariables|SetSegmentLength (Utilities|Select :Index (Variables|ArraySettings|GetSplineMeshForwardAxis) :X (.x (Variables|ArraySettings|GetSegmentSpaceBound)) :Y (.y (Variables|ArraySettings|GetSegmentSpaceBound)) :Z (.z (Variables|ArraySettings|GetSegmentSpaceBound))))
      (switch Utilities|FlowControl|Switch|SwitchonEStaticMeshArrayMode (Variables|ArraySettings|GetArrayMode)
        (:NewEnumerator0
          ;[1 1 0] 这个是直接用控制点来生成平铺阵列
          (for _index (range 0 (Math|Float|Truncate (/ (Math|Float|Absolute(Float) (.x _handlepoint)) (.x (Variables|ArraySettings|GetSegmentSpaceBound)))))
            (for _index_2 (range 0 (Math|Float|Truncate (/ (Math|Float|Absolute(Float) (.y _handlepoint)) (.y (Variables|ArraySettings|GetSegmentSpaceBound)))))
              (for _index_3 (range 0 (Math|Float|Truncate (/ (Math|Float|Absolute(Float) (.z _handlepoint)) (.z (Variables|ArraySettings|GetSegmentSpaceBound)))))
                (bind _returnvalue_2 (AddComponent|AddStaticMeshComponent false (Math|Transform|MakeTransform (Math|Vector|MakeVector (* (Math|Conversions|ToFloat(Integer) _index) (Math|Float|Sign(Float) (.x _handlepoint)) (.x (Variables|ArraySettings|GetSegmentSpaceBound))) (* (Math|Conversions|ToFloat(Integer) _index_2) (Math|Float|Sign(Float) (.y _handlepoint)) (.y (Variables|ArraySettings|GetSegmentSpaceBound))) (* (Math|Conversions|ToFloat(Integer) _index_3) (Math|Float|Sign(Float) (.z _handlepoint)) (.z (Variables|ArraySettings|GetSegmentSpaceBound)))) "0, 0, 0" "1,1,1")))
                (Components|StaticMesh|SetStaticMesh _returnvalue_2 (Variables|ArraySettings|GetStaticMesh))))))
        (:NewEnumerator1
          ;[1 1 0] 直接沿着Spline生成队列，但是并不完全拟合Spline
          (for _index_4 (range 0 (Math|Float|Truncate (/ (Spline|GetSplineLength (Variables|Default|GetSpline)) (LocalVariables|GetSegmentLength))))
            (bind _returnvalue_3 (AddComponent|AddStaticMeshComponent false (Spline|GetTransformatDistanceAlongSpline (Variables|Default|GetSpline) (* _index_4 (LocalVariables|GetSegmentLength)) "Local" false)))
            (Components|StaticMesh|SetStaticMesh _returnvalue_3 (Variables|ArraySettings|GetStaticMesh))))
        (:NewEnumerator3
          ;[1 1 0] 完全拟合Spline的模式，N个Spline控制点产生N-1段SplineMesh
          (for _index_5 (range 0 (- (Spline|GetNumberOfSplinePoints (Variables|Default|GetSpline)) 2))
            (bind _returnvalue_4 (AddComponent|AddSplineMeshComponent false))
            (Components|StaticMesh|SetStaticMesh _returnvalue_4 (Variables|ArraySettings|GetStaticMesh))
            (SplineMesh|SetForwardAxis _returnvalue_4 (Variables|ArraySettings|GetSplineMeshForwardAxis) true)
            (SplineMesh|SetStartandEnd _returnvalue_4 (.Location (Spline|GetLocationandTangentatSplinePoint _spline_2 _index_5 "Local")) (.Tangent (Spline|GetLocationandTangentatSplinePoint _spline_2 _index_5 "Local")) (.Location (Spline|GetLocationandTangentatSplinePoint _spline_2 (+ _index_5 1) "Local")) (.Tangent (Spline|GetLocationandTangentatSplinePoint _spline_2 (+ _index_5 1) "Local")) true :!class /Script/Engine.SplineMeshComponent)
            (SplineMesh|SetStartScale _returnvalue_4 (Math|Vector2D|MakeVector2D _thickness _thickness) true :!class /Script/Engine.SplineMeshComponent)
            (SplineMesh|SetEndScale _returnvalue_4 (Math|Vector2D|MakeVector2D _thickness_2 _thickness_2) true :!class /Script/Engine.SplineMeshComponent)))
        (:NewEnumerator2
          ;[1 1 0] 这个是让模型队形相对比较贴合Spline，每个SplineMesh分段都是自动均匀分布，在某些曲度比较大的地方可能不会贴合Spline
          (for _index_6 (range 0 (- (Math|Float|Truncate (/ (Spline|GetSplineLength (Variables|Default|GetSpline)) (LocalVariables|GetSegmentLength))) 1))
            (bind _returnvalue_5 (AddComponent|AddSplineMeshComponent false))
            (Components|StaticMesh|SetStaticMesh _returnvalue_5 (Variables|ArraySettings|GetStaticMesh))
            (SplineMesh|SetForwardAxis _returnvalue_5 (Variables|ArraySettings|GetSplineMeshForwardAxis) true)
            (SplineMesh|SetStartandEnd _returnvalue_5 (Spline|GetLocationatDistanceAlongSpline _spline (* _index_6 (LocalVariables|GetSegmentLength)) "Local") (* (Spline|GetDirectionatDistanceAlongSpline _spline (* _index_6 (LocalVariables|GetSegmentLength)) "Local") (LocalVariables|GetSegmentLength)) (Spline|GetLocationatDistanceAlongSpline _spline (* (+ _index_6 1) (LocalVariables|GetSegmentLength)) "Local") (* (Spline|GetDirectionatDistanceAlongSpline _spline (* (+ _index_6 1) (LocalVariables|GetSegmentLength)) "Local") (LocalVariables|GetSegmentLength)) true :!class /Script/Engine.SplineMeshComponent)
            (SplineMesh|SetStartScale _returnvalue_5 (Math|Vector2D|MakeVector2D _thickness_3 _thickness_3) true :!class /Script/Engine.SplineMeshComponent)
            (SplineMesh|SetEndScale _returnvalue_5 (Math|Vector2D|MakeVector2D _thickness_4 _thickness_4) true :!class /Script/Engine.SplineMeshComponent)))))))
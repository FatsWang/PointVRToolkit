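; Transform gizmo actor with translation, rotation and scale handle sets, starting in Rotation mode and rescaling with camera distance.
; A map tags each handle with mode, orientation and axis, driving hover materials and drag setup.
; Only trackball dragging is implemented: the mouse ray hits a camera-facing plane, projects onto a virtual sphere, and successive vectors yield delta rotations for TransformedObjectRoot, which the actor's rotation follows.
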(event EventBeginPlay
  (CallFunction|SwitchTransformMode "NewEnumerator1"))

(event EventTick
  (params (DeltaSeconds :type Float%20%28single-precision%29))
  (CallFunction|UpdateGizmoScale))

(fn ConstructionScript
  (CallFunction|SwitchTransformMode "NewEnumerator1")
  (CallFunction|InitialTransformHandleIdentity))

(fn SwitchTransformMode
  (params (TransformMode :type ETransformMode%20Enum :default "NewEnumerator0"))
  (switch Utilities|FlowControl|Switch|SwitchonETransformMode TransformMode
    (:NewEnumerator0
      (Translation|SetActiveTranslationGizmo true)
      (Rotation|SetActiveRotationGizmo false)
      (Scale|SetActiveScaleGizmo false))
    (:NewEnumerator1
      (Translation|SetActiveTranslationGizmo false)
      (Rotation|SetActiveRotationGizmo true)
      (Scale|SetActiveScaleGizmo false))
    (:NewEnumerator2
      (Translation|SetActiveTranslationGizmo false)
      (Rotation|SetActiveRotationGizmo false)
      (Scale|SetActiveScaleGizmo true))))

(fn SetActiveRotationGizmo
  (params (NewActive :type Boolean))
  (bind _trackballhandle (Variables|TransformHandle|GetTrackBallHandle))
  (Rendering|SetVisibility (Variables|Default|GetRotationGizmoRoot) NewActive true)
  (if NewActive
    (Collision|SetCollisionEnabled _trackballhandle "QueryOnly")
    (else
      (Collision|SetCollisionEnabled _trackballhandle "NoCollision"))))

(fn SetActiveScaleGizmo
  (params (NewActive :type Boolean))
  (bind _uniformscalehandle (Variables|TransformHandle|GetUniformScaleHandle))
  (Rendering|SetVisibility (Variables|Default|GetScaleGizmoRoot) NewActive true)
  (if NewActive
    (Collision|SetCollisionEnabled _uniformscalehandle "QueryOnly")
    (else
      (Collision|SetCollisionEnabled _uniformscalehandle "NoCollision"))))

(fn SetActiveTranslationGizmo
  (params (NewActive :type Boolean))
  (bind _freetranslationhandle (Variables|TransformHandle|GetFreeTranslationHandle))
  (Rendering|SetVisibility (Variables|Default|GetTranslationGizmoRoot) NewActive true)
  (if NewActive
    (Collision|SetCollisionEnabled _freetranslationhandle "QueryOnly")
    (else
      (Collision|SetCollisionEnabled _freetranslationhandle "NoCollision"))))

(fn UpdateGizmoScale
  (bind _returnvalue (Game|GetPlayerCameraManager 0))
  (bind _returnvalue_2 (Transformation|GetActorLocation))
  (bind _gizmoscale (Variables|Default|GetGizmoScale))
  (bind _returnvalue_3 (Camera|GetCameraLocation _returnvalue))
  (bind _returnvalue_4 (Math|Vector|Distance(Vector) _returnvalue_3 _returnvalue_2))
  (bind _returnvalue_5 (/ _returnvalue_4 5e+02))
  (bind _returnvalue_6 (* _returnvalue_5 _gizmoscale))
  (Transformation|SetActorScale3D (Math|Conversions|ToVector(Float) _returnvalue_6))
  (Variables|Default|SetTrackballRadius (* _returnvalue_6 5e+01)))

(fn InitialTransformHandleIdentity
  (bind _transformhandleidentity (Variables|Default|GetTransformHandleIdentity))
  (Utilities|Map|Clear _transformhandleidentity) ; 拖动Actor的时候构造脚本会持续运行，填充大量垃圾数据，不清楚运行时会不会自动清空这些无用数据，我这里保险起见先清空了
  ;[1 1 0] Translation移动
  (Utilities|Map|Add _transformhandleidentity (Variables|TransformHandle|GetFreeTranslationHandle) (Utilities|Struct|MakeSTransformHandleIdentity "NewEnumerator0" "NewEnumerator1" "NewEnumerator8"))
  (Utilities|Map|Add _transformhandleidentity (Variables|TransformHandle|GetTranslationHandleXAxis) (Utilities|Struct|MakeSTransformHandleIdentity "NewEnumerator0" "NewEnumerator1" "NewEnumerator0"))
  (Utilities|Map|Add _transformhandleidentity (Variables|TransformHandle|GetTranslationHandleYAxis) (Utilities|Struct|MakeSTransformHandleIdentity "NewEnumerator0" "NewEnumerator1" "NewEnumerator1"))
  (Utilities|Map|Add _transformhandleidentity (Variables|TransformHandle|GetTranslationHandleZAxis) (Utilities|Struct|MakeSTransformHandleIdentity "NewEnumerator0" "NewEnumerator1" "NewEnumerator2"))
  (Utilities|Map|Add _transformhandleidentity (Variables|Default|GetTranslationHandleYZAxis) (Utilities|Struct|MakeSTransformHandleIdentity "NewEnumerator0" "NewEnumerator1" "NewEnumerator11"))
  (Utilities|Map|Add _transformhandleidentity (Variables|Default|GetTranslationHandleXZAxis) (Utilities|Struct|MakeSTransformHandleIdentity "NewEnumerator0" "NewEnumerator1" "NewEnumerator10"))
  (Utilities|Map|Add _transformhandleidentity (Variables|Default|GetTranslationHandleXYAxis) (Utilities|Struct|MakeSTransformHandleIdentity "NewEnumerator0" "NewEnumerator1" "NewEnumerator9"))
  ;[1 1 0] Rotation旋转，目前我旋转只有Local坐标系下执行
  (Utilities|Map|Add _transformhandleidentity (Variables|TransformHandle|GetTrackBallHandle) (Utilities|Struct|MakeSTransformHandleIdentity "NewEnumerator1" "NewEnumerator0" "NewEnumerator8"))
  (Utilities|Map|Add _transformhandleidentity (Variables|TransformHandle|GetRotationHandleXAxis) (Utilities|Struct|MakeSTransformHandleIdentity "NewEnumerator1" "NewEnumerator0" "NewEnumerator0"))
  (Utilities|Map|Add _transformhandleidentity (Variables|TransformHandle|GetRotationHandleYAxis) (Utilities|Struct|MakeSTransformHandleIdentity "NewEnumerator1" "NewEnumerator0" "NewEnumerator1"))
  (Utilities|Map|Add _transformhandleidentity (Variables|TransformHandle|GetRotationHandleZAxis) (Utilities|Struct|MakeSTransformHandleIdentity "NewEnumerator1" "NewEnumerator0" "NewEnumerator2"))
  ;[1 1 0] Scale缩放，缩放一般也只有在Local坐标系下执行
  (Utilities|Map|Add _transformhandleidentity (Variables|TransformHandle|GetUniformScaleHandle) (Utilities|Struct|MakeSTransformHandleIdentity "NewEnumerator2" "NewEnumerator0" "NewEnumerator8"))
  (Utilities|Map|Add _transformhandleidentity (Variables|TransformHandle|GetScaleHandleXAxis) (Utilities|Struct|MakeSTransformHandleIdentity "NewEnumerator2" "NewEnumerator0" "NewEnumerator0"))
  (Utilities|Map|Add _transformhandleidentity (Variables|TransformHandle|GetScaleHandleYAxis) (Utilities|Struct|MakeSTransformHandleIdentity "NewEnumerator2" "NewEnumerator0" "NewEnumerator1"))
  (Utilities|Map|Add _transformhandleidentity (Variables|TransformHandle|GetScaleHandleZAxis) (Utilities|Struct|MakeSTransformHandleIdentity "NewEnumerator2" "NewEnumerator0" "NewEnumerator2"))
  (Utilities|Map|Add _transformhandleidentity (Variables|Default|GetScaleHandleYZAxis) (Utilities|Struct|MakeSTransformHandleIdentity "NewEnumerator2" "NewEnumerator0" "NewEnumerator11"))
  (Utilities|Map|Add _transformhandleidentity (Variables|Default|GetScaleHandleXZAxis) (Utilities|Struct|MakeSTransformHandleIdentity "NewEnumerator2" "NewEnumerator0" "NewEnumerator10"))
  (Utilities|Map|Add _transformhandleidentity (Variables|Default|GetScaleHandleXYAxis) (Utilities|Struct|MakeSTransformHandleIdentity "NewEnumerator2" "NewEnumerator0" "NewEnumerator9")))

(fn DeprojectPlanetoTrackball
  (bind _returnvalue (Game|GetPlayerController 0))
  (bind _cameratransform (Variables|Default|GetCameraTransform))
  (bind _trackballradius (Variables|Default|GetTrackballRadius))
  (bind _returnvalue_2 (Math|Float|Square _trackballradius))
  (bind (_locationx _locationy) (Game|Player|GetMousePosition _returnvalue))
  (bind (_worldlocation _worlddirection) (Class|PlayerController|DeprojectScreenPositiontoWorld _returnvalue _locationx _locationy))
  (LocalVariables|SetIntersectPointInCameraSpace (Math|Transform|InverseTransformLocation _cameratransform (.Intersection (Class|KismetMathLibrary|LinePlaneIntersection _worldlocation (+ _worldlocation (* _worlddirection 1e+04)) (Variables|Default|GetVirtualPlane)))))
  (LocalVariables|SetTrackballCenterInCameraSpace (Math|Transform|InverseTransformLocation _cameratransform (Transformation|GetActorLocation)))
  (if (>= _returnvalue_2 (+ (Math|Float|Square (.y (- (LocalVariables|GetIntersectPointInCameraSpace) (LocalVariables|GetTrackballCenterInCameraSpace)))) (Math|Float|Square (.z (- (LocalVariables|GetIntersectPointInCameraSpace) (LocalVariables|GetTrackballCenterInCameraSpace))))))
    (return (Math|Vector|Normalize (+ (* (Math|Vector|NegateVector (Class|KismetMathLibrary|VectorForward)) (Math|Float|Sqrt (- _returnvalue_2 (+ (Math|Float|Square (.y (- (LocalVariables|GetIntersectPointInCameraSpace) (LocalVariables|GetTrackballCenterInCameraSpace)))) (Math|Float|Square (.z (- (LocalVariables|GetIntersectPointInCameraSpace) (LocalVariables|GetTrackballCenterInCameraSpace)))))))) (Math|Vector|MakeVector 0.0 (.y (- (LocalVariables|GetIntersectPointInCameraSpace) (LocalVariables|GetTrackballCenterInCameraSpace))) (.z (- (LocalVariables|GetIntersectPointInCameraSpace) (LocalVariables|GetTrackballCenterInCameraSpace)))))))
    (else
      (return (Math|Vector|Normalize (Math|Vector|MakeVector 0.0 (.y (- (LocalVariables|GetIntersectPointInCameraSpace) (LocalVariables|GetTrackballCenterInCameraSpace))) (.z (- (LocalVariables|GetIntersectPointInCameraSpace) (LocalVariables|GetTrackballCenterInCameraSpace)))))))))

(fn CalculateTrackballDeltaRotation
  (params (PreviousProjectionVector :type Vector) (CurrentProjectionVector :type Vector))
  (return (Math|Vector|RotatorfromAxisandAngle (Math|Transform|TransformDirection (Variables|Default|GetCameraTransform) (Math|Vector|CrossProduct PreviousProjectionVector CurrentProjectionVector)) (Class|KismetMathLibrary|DegAcos (Math|Vector|DotProduct PreviousProjectionVector CurrentProjectionVector)))))

(fn ApplyTrackballRotation
  (params (DeltaRotation :type Rotator))
  (bind _transformedobjectroot (Variables|Default|GetTransformedObjectRoot))
  (Transformation|AddWorldRotation _transformedobjectroot DeltaRotation false false)
  (Transformation|SetActorRotation (Transformation|GetWorldRotation _transformedobjectroot)))

(fn OnClickPressed
  (params (Interactor :type BPC%20Toolkit%20Trace%20Interactor%20Object%20Reference) (TraceHit :type Hit%20Result%20Structure%20%28by%20ref%29))
  (return false))

(fn OnClickReleased
  (params (Interactor :type BPC%20Toolkit%20Trace%20Interactor%20Object%20Reference) (TraceHit :type Hit%20Result%20Structure%20%28by%20ref%29))
  (return false))

(fn OnComponentHovered
  (params (Interactor :type BPC%20Toolkit%20Trace%20Interactor%20Object%20Reference) (TraceHit :type Hit%20Result%20Structure%20%28by%20ref%29) (CurrentComponent :type Primitive%20Component%20Object%20Reference))
  (bind _transformhandleidentity (Variables|Default|GetTransformHandleIdentity))
  (bind _value (Utilities|Map|Find _transformhandleidentity CurrentComponent))
  (switch Utilities|FlowControl|Switch|SwitchonETransformMode (.transformmode _value)
    (:NewEnumerator0
      (Rendering|Material|SetMaterial CurrentComponent 0 "/Game/PointVRToolkit/Materials/TransformGizmo/MI_Hovered.MI_Hovered" :!label _label))
    (:NewEnumerator1
      (switch Utilities|FlowControl|Switch|SwitchonEConstraintAxis (.constraintaxis _value)
        (:NewEnumerator0
          (Rendering|Material|SetMaterial CurrentComponent 0 "/Game/PointVRToolkit/Materials/TransformGizmo/MI_Rotation_Hovered.MI_Rotation_Hovered" :!label _label_2))
        (:NewEnumerator1
          (goto _label_2))
        (:NewEnumerator2
          (goto _label_2))
        (:NewEnumerator8
          (Rendering|Material|SetMaterial CurrentComponent 0 "/Game/PointVRToolkit/Materials/TransformGizmo/MI_Trackball_Hovered.MI_Trackball_Hovered"))))
    (:NewEnumerator2
      (goto _label)))
  (return false))

(fn OnComponentUnhovered
  (params (Interactor :type BPC%20Toolkit%20Trace%20Interactor%20Object%20Reference) (TraceHit :type Hit%20Result%20Structure%20%28by%20ref%29) (PreviousComponent :type Primitive%20Component%20Object%20Reference))
  (bind _transformhandleidentity (Variables|Default|GetTransformHandleIdentity))
  (bind _value (Utilities|Map|Find _transformhandleidentity PreviousComponent))
  (switch Utilities|FlowControl|Switch|SwitchonETransformMode (.transformmode _value)
    (:NewEnumerator0
      (switch Utilities|FlowControl|Switch|SwitchonEConstraintAxis (.constraintaxis _value) :!label _label
        (:NewEnumerator0
          (Rendering|Material|SetMaterial PreviousComponent 0 "/Game/PointVRToolkit/Materials/TransformGizmo/MI_XAxis.MI_XAxis" :!label _label_2))
        (:NewEnumerator1
          (Rendering|Material|SetMaterial PreviousComponent 0 "/Game/PointVRToolkit/Materials/TransformGizmo/MI_YAxis.MI_YAxis" :!label _label_3))
        (:NewEnumerator2
          (Rendering|Material|SetMaterial PreviousComponent 0 "/Game/PointVRToolkit/Materials/TransformGizmo/MI_ZAxis.MI_ZAxis" :!label _label_4))
        (:NewEnumerator11
          (goto _label_2))
        (:NewEnumerator10
          (goto _label_3))
        (:NewEnumerator9
          (goto _label_4))
        (:NewEnumerator8
          (Rendering|Material|SetMaterial PreviousComponent 0 "/Game/PointVRToolkit/Materials/TransformGizmo/MI_XYZAxis.MI_XYZAxis"))))
    (:NewEnumerator1
      (switch Utilities|FlowControl|Switch|SwitchonEConstraintAxis (.constraintaxis _value)
        (:NewEnumerator0
          (Rendering|Material|SetMaterial PreviousComponent 0 "/Game/PointVRToolkit/Materials/TransformGizmo/MI_Rotation_XAxis.MI_Rotation_XAxis"))
        (:NewEnumerator1
          (Rendering|Material|SetMaterial PreviousComponent 0 "/Game/PointVRToolkit/Materials/TransformGizmo/MI_Rotation_YAxis.MI_Rotation_YAxis"))
        (:NewEnumerator2
          (Rendering|Material|SetMaterial PreviousComponent 0 "/Game/PointVRToolkit/Materials/TransformGizmo/MI_Rotation_ZAxis.MI_Rotation_ZAxis"))
        (:NewEnumerator8
          (Rendering|Material|SetMaterial PreviousComponent 0 "/Game/PointVRToolkit/Materials/TransformGizmo/MI_TrackBall.MI_TrackBall"))))
    (:NewEnumerator2
      (goto _label)))
  (return false))

(fn OnDragCanceled
  (params (Interactor :type BPC%20Toolkit%20Trace%20Interactor%20Object%20Reference) (TraceHit :type Hit%20Result%20Structure%20%28by%20ref%29))
  (Default|UnlockHovered Interactor)
  (return false))

(fn OnDragDetected
  (params (Interactor :type BPC%20Toolkit%20Trace%20Interactor%20Object%20Reference) (TraceHit :type Hit%20Result%20Structure%20%28by%20ref%29))
  (bind _hitcomponent (Collision|BreakHitResult TraceHit))
  (bind _transformhandleidentity (Variables|Default|GetTransformHandleIdentity))
  (bind _value (Utilities|Map|Find _transformhandleidentity _hitcomponent))
  (Default|LockHovered Interactor)
  (Variables|Default|SetCameraTransform (Transformation|GetActorTransform (Game|GetPlayerCameraManager 0)))
  (Variables|Default|SetTransformMode (.transformmode _value))
  (Variables|Default|SetOrientType (.orienttype _value))
  (Variables|Default|SetConstraintAxis (.constraintaxis _value))
  (switch Utilities|FlowControl|Switch|SwitchonETransformMode (Variables|Default|GetTransformMode)
    (:NewEnumerator1
      (switch Utilities|FlowControl|Switch|SwitchonEConstraintAxis (Variables|Default|GetConstraintAxis)
        (:NewEnumerator8
          ;[1 1 0] Trackball
          (Variables|Default|SetVirtualPlane (Class|KismetMathLibrary|MakePlanefromPointandNormal (Transformation|GetActorLocation) (Math|Transform|TransformDirection (Variables|Default|GetCameraTransform) (Class|KismetMathLibrary|VectorForward))))
          (bind _outvector (Rotation|DeprojectPlanetoTrackball))
          (bind _output_get (Variables|Default|SetPreviousTrackballProjectionVector _outvector))
          (Variables|Default|SetCurrentTrackballProjectionVector _output_get)
          (return true))))))

(fn OnDragMove
  (params (Interactor :type BPC%20Toolkit%20Trace%20Interactor%20Object%20Reference) (TraceHit :type Hit%20Result%20Structure%20%28by%20ref%29))
  (switch Utilities|FlowControl|Switch|SwitchonETransformMode (Variables|Default|GetTransformMode)
    (:NewEnumerator1
      (switch Utilities|FlowControl|Switch|SwitchonEConstraintAxis (Variables|Default|GetConstraintAxis)
        (:NewEnumerator8
          (bind _outvector (Rotation|DeprojectPlanetoTrackball))
          (Variables|Default|SetCurrentTrackballProjectionVector _outvector)
          (bind _deltarotation (Rotation|CalculateTrackballDeltaRotation (Variables|Default|GetPreviousTrackballProjectionVector) (Variables|Default|GetCurrentTrackballProjectionVector)))
          (Rotation|ApplyTrackballRotation _deltarotation)
          (Variables|Default|SetPreviousTrackballProjectionVector (Variables|Default|GetCurrentTrackballProjectionVector))
          (return false))))))

(fn OnTraceEnter
  (params (Interactor :type BPC%20Toolkit%20Trace%20Interactor%20Object%20Reference) (TraceHit :type Hit%20Result%20Structure%20%28by%20ref%29))
  (return false))

(fn OnTraceLeave
  (params (Interactor :type BPC%20Toolkit%20Trace%20Interactor%20Object%20Reference) (TraceHit :type Hit%20Result%20Structure%20%28by%20ref%29))
  (return false))

(fn OnTraceMove
  (params (Interactor :type BPC%20Toolkit%20Trace%20Interactor%20Object%20Reference) (TraceHit :type Hit%20Result%20Structure%20%28by%20ref%29))
  (return false))
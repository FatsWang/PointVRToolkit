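; Transform gizmo for the PointVR Toolkit that moves, rotates and uniformly resizes a TransformedObject through draggable, hover-highlighted handles, keeping its size proportional to camera distance.
; A map built in the construction script gives each handle its mode and axis, read when a drag starts.
; Translate and rotate intersect the mouse ray with a virtual plane to get per-frame world-axis offsets or arcball angles.
; Resize uses raw mouse delta, and translation re-centers the gizmo on the object.
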(event Custom|RotateObject
  (params (Axis :type EConstraintAxis%20Enum :default "NewEnumerator0") (DeltaAngle :type Float%20%28single-precision%29))
  (bind _transformedobject (Variables|Default|GetTransformedObject))
  (switch Utilities|FlowControl|Switch|SwitchonEConstraintAxis Axis
    (:NewEnumerator0
      (Class|Actor|AddActorWorldRotation _transformedobject (Math|Rotator|MakeRotator DeltaAngle 0.0 0.0)))
    (:NewEnumerator1
      (Class|Actor|AddActorWorldRotation _transformedobject (Math|Rotator|MakeRotator 0.0 DeltaAngle 0.0)))
    (:NewEnumerator2
      (Class|Actor|AddActorWorldRotation _transformedobject (Math|Rotator|MakeRotator 0.0 0.0 DeltaAngle)))))

(event Custom|TranslateObject
  (params (Axis :type EConstraintAxis%20Enum :default "NewEnumerator0") (DeltaLocation :type Vector))
  (bind (_x _y _z) (Math|Vector|BreakVector DeltaLocation))
  (bind _transformedobject (Variables|Default|GetTransformedObject))
  (switch Utilities|FlowControl|Switch|SwitchonEConstraintAxis Axis
    (:NewEnumerator0
      (Transformation|AddActorWorldOffset _transformedobject (Math|Vector|MakeVector _x 0.0 0.0)))
    (:NewEnumerator1
      (Transformation|AddActorWorldOffset _transformedobject (Math|Vector|MakeVector 0.0 _y 0.0)))
    (:NewEnumerator2
      (Transformation|AddActorWorldOffset _transformedobject (Math|Vector|MakeVector 0.0 0.0 _z))))
  (Transformation|SetActorLocation (Transformation|GetActorLocation (Variables|Default|GetTransformedObject)) false false))

(event Custom|ResizeObject
  (params (DeltaScale :type Vector))
  (CallFunction|AddActorWorldScale (Variables|Default|GetTransformedObject) DeltaScale))

(event EventBeginPlay)

(event Collision|EventActorBeginOverlap
  (params (OtherActor :type Actor%20Object%20Reference)))

(event EventTick
  (params (DeltaSeconds :type Float%20%28single-precision%29))
  (Transformation|SetActorScale3D (Math|Conversions|ToVector(Float) (/ (Math|Vector|Distance(Vector) (Camera|GetCameraLocation (Game|GetPlayerCameraManager 0)) (Transformation|GetActorLocation)) 2e+02))))

(fn ConstructionScript
  (bind _transformenum (Variables|Default|GetTransformEnum))
  (Utilities|Map|Clear _transformenum)
  (Utilities|Map|Add _transformenum (Variables|Default|GetTranslateHandle_X) (Utilities|Struct|MakeStruct_TransformEnum "NewEnumerator0" "NewEnumerator0"))
  (Utilities|Map|Add _transformenum (Variables|Default|GetTranslateHandle_Y) (Utilities|Struct|MakeStruct_TransformEnum "NewEnumerator0" "NewEnumerator1"))
  (Utilities|Map|Add _transformenum (Variables|Default|GetTranslateHandle_Z) (Utilities|Struct|MakeStruct_TransformEnum "NewEnumerator0" "NewEnumerator2"))
  (Utilities|Map|Add _transformenum (Variables|Default|GetRotateHandle_X) (Utilities|Struct|MakeStruct_TransformEnum "NewEnumerator1" "NewEnumerator0"))
  (Utilities|Map|Add _transformenum (Variables|Default|GetRotateHandle_Y) (Utilities|Struct|MakeStruct_TransformEnum "NewEnumerator1" "NewEnumerator1"))
  (Utilities|Map|Add _transformenum (Variables|Default|GetRotateHandle_Z) (Utilities|Struct|MakeStruct_TransformEnum "NewEnumerator1" "NewEnumerator2"))
  (Utilities|Map|Add _transformenum (Variables|Default|GetUniformResizeHandle) (Utilities|Struct|MakeStruct_TransformEnum "NewEnumerator2" "NewEnumerator8")))

(fn OnClickPressed
  (params (Interactor :type BPC%20Toolkit%20Trace%20Interactor%20Object%20Reference) (TraceHit :type Hit%20Result%20Structure%20%28by%20ref%29))
  (return false))

(fn OnClickReleased
  (params (Interactor :type BPC%20Toolkit%20Trace%20Interactor%20Object%20Reference) (TraceHit :type Hit%20Result%20Structure%20%28by%20ref%29))
  (return false))

(fn OnComponentHovered
  (params (Interactor :type BPC%20Toolkit%20Trace%20Interactor%20Object%20Reference) (TraceHit :type Hit%20Result%20Structure%20%28by%20ref%29) (CurrentComponent :type Primitive%20Component%20Object%20Reference))
  (Rendering|Material|SetMaterial CurrentComponent 0 "/Game/PointVRToolkit/Materials/Gizmo/MI_HoveredGIzmo.MI_HoveredGizmo")
  (return false))

(fn OnComponentUnhovered
  (params (Interactor :type BPC%20Toolkit%20Trace%20Interactor%20Object%20Reference) (TraceHit :type Hit%20Result%20Structure%20%28by%20ref%29) (PreviousComponent :type Primitive%20Component%20Object%20Reference))
  (switch Utilities|FlowControl|Switch|SwitchonEConstraintAxis (.transformaxis (.Value (Utilities|Map|Find (Variables|Default|GetTransformEnum) PreviousComponent)))
    (:NewEnumerator0
      (Rendering|Material|SetMaterial PreviousComponent 0 "/Game/PointVRToolkit/Materials/Gizmo/MI_XAxis.MI_XAxis"))
    (:NewEnumerator1
      (Rendering|Material|SetMaterial PreviousComponent 0 "/Game/PointVRToolkit/Materials/Gizmo/MI_YAxis.MI_YAxis"))
    (:NewEnumerator2
      (Rendering|Material|SetMaterial PreviousComponent 0 "/Game/PointVRToolkit/Materials/Gizmo/MI_ZAxis.MI_ZAxis"))
    (:NewEnumerator8
      (Rendering|Material|SetMaterial PreviousComponent 0 "/Game/PointVRToolkit/Materials/Gizmo/MI_XYZAxis.MI_XYZAxis")))
  (return false))

(fn OnDragCanceled
  (params (Interactor :type BPC%20Toolkit%20Trace%20Interactor%20Object%20Reference) (TraceHit :type Hit%20Result%20Structure%20%28by%20ref%29))
  (Default|UnlockHovered Interactor)
  (return false))

(fn OnDragDetected
  (params (Interactor :type BPC%20Toolkit%20Trace%20Interactor%20Object%20Reference) (TraceHit :type Hit%20Result%20Structure%20%28by%20ref%29))
  (bind _returnvalue (Game|GetPlayerCameraManager 0))
  (bind _returnvalue_2 (Transformation|GetActorLocation))
  (bind (_bblockinghit _binitialoverlap _time _distance _location _impactpoint _normal _impactnormal _physmat _hitactor _hitcomponent) (Collision|BreakHitResult TraceHit))
  (bind _transformenum (Variables|Default|GetTransformEnum))
  (bind (_x _y _z) (Math|Vector|BreakVector _returnvalue_2))
  (bind _value (Utilities|Map|Find _transformenum _hitcomponent))
  (bind (_x_2 _y_2 _z_2) (Math|Vector|BreakVector _returnvalue_2))
  (bind _returnvalue_3 (Camera|GetCameraRotation _returnvalue))
  (bind (_x_3 _y_3) (Math|Vector|BreakVector _returnvalue_2))
  (bind _returnvalue_4 (Math|Vector|GetForwardVector _returnvalue_3))
  (bind _returnvalue_5 (Math|Vector|ProjectVectorontoPlane _returnvalue_4 "0, 0,1.000000"))
  (bind _returnvalue_6 (Math|Vector|ProjectVectorontoPlane _returnvalue_4 "1.000000, 0, 0"))
  (bind _returnvalue_7 (Math|Vector|ProjectVectorontoPlane _returnvalue_4 "0.000000,1.000000, 0"))
  (bind _returnvalue_8 (Math|Vector|Normalize _returnvalue_6))
  (bind _returnvalue_9 (Math|Vector|Normalize _returnvalue_5))
  (bind _returnvalue_10 (Math|Vector|Normalize _returnvalue_7))
  (bind (_x_4 _y_4) (Math|Vector|BreakVector _returnvalue_9))
  (bind (_x_5 _y_5 _z_3) (Math|Vector|BreakVector _returnvalue_10))
  (bind (_x_6 _y_6 _z_4) (Math|Vector|BreakVector _returnvalue_8))
  (Default|LockHovered Interactor)
  (bind _output_get (Variables|Default|SetDragDetectedLocation _impactpoint))
  (bind _output_get_2 (Variables|Default|SetCurrentFrameDragLocation _output_get))
  (Variables|Default|SetPreviousFrameDragLocation _output_get_2)
  (Variables|Default|SetTransformMode (.transformtype _value))
  (Variables|Default|SetConstraintAxis (.transformaxis _value))
  (switch Utilities|FlowControl|Switch|SwitchonETransformMode (Variables|Default|GetTransformMode)
    (:NewEnumerator0
      ;[1 1 0] 平移部分
      (switch Utilities|FlowControl|Switch|SwitchonEConstraintAxis (Variables|Default|GetConstraintAxis)
        (:NewEnumerator0
          (Variables|Default|SetVirtualPlane (Class|KismetMathLibrary|MakePlanefromPointandNormal (Variables|Default|GetDragDetectedLocation) (Math|Vector|SelectVector "0,1.000000, 0" "0, 0,1.000000" (>= (Math|Float|Absolute(Float) _y_6) (Math|Float|Absolute(Float) _z_4))))))
        (:NewEnumerator1
          (Variables|Default|SetVirtualPlane (Class|KismetMathLibrary|MakePlanefromPointandNormal (Variables|Default|GetDragDetectedLocation) (Math|Vector|SelectVector "1.000000, 0, 0" "0, 0,1.000000" (>= (Math|Float|Absolute(Float) _x_5) (Math|Float|Absolute(Float) _z_3))))))
        (:NewEnumerator2
          (Variables|Default|SetVirtualPlane (Class|KismetMathLibrary|MakePlanefromPointandNormal (Variables|Default|GetDragDetectedLocation) (Math|Vector|SelectVector "1.000000, 0, 0" "0,1.000000, 0" (>= (Math|Float|Absolute(Float) _x_4) (Math|Float|Absolute(Float) _y_4))))))
        (:NewEnumerator8
          (return false)))
      (return true))
    (:NewEnumerator1
      ;[1 1 0] 旋转部分
      (switch Utilities|FlowControl|Switch|SwitchonEConstraintAxis (Variables|Default|GetConstraintAxis)
        (:NewEnumerator0
          (Variables|Default|SetVirtualPlane (Class|KismetMathLibrary|MakePlanefromPointandNormal (Math|Vector|MakeVector (.X (Math|Vector|BreakVector (Variables|Default|GetDragDetectedLocation))) _y _z) "1.000000, 0,0.000000")))
        (:NewEnumerator1
          (Variables|Default|SetVirtualPlane (Class|KismetMathLibrary|MakePlanefromPointandNormal (Math|Vector|MakeVector _x_2 (.Y (Math|Vector|BreakVector (Variables|Default|GetDragDetectedLocation))) _z_2) "0.000000,1.000000,0.000000")))
        (:NewEnumerator2
          (Variables|Default|SetVirtualPlane (Class|KismetMathLibrary|MakePlanefromPointandNormal (Math|Vector|MakeVector _x_3 _y_3 (.Z (Math|Vector|BreakVector (Variables|Default|GetDragDetectedLocation)))) "0, 0,1.000000")))
        (:NewEnumerator8
          (return false)))
      (return true))
    (:NewEnumerator2
      (return true))))

(fn OnDragMove
  (params (Interactor :type BPC%20Toolkit%20Trace%20Interactor%20Object%20Reference) (TraceHit :type Hit%20Result%20Structure%20%28by%20ref%29))
  (bind _returnvalue (Game|GetPlayerController 0))
  (bind _returnvalue_2 (Game|GetPlayerController 0))
  (bind _returnvalue_3 (Transformation|GetActorLocation))
  (bind _virtualplane (Variables|Default|GetVirtualPlane))
  (bind _constraintaxis (Variables|Default|GetConstraintAxis))
  (bind (_deltax _deltay) (Class|PlayerController|GetInputMouseDelta _returnvalue_2))
  (bind (_worldlocation _worlddirection) (Game|Player|ConvertMouseLocationToWorldSpace _returnvalue))
  (bind _returnvalue_4 (* _worlddirection 1e+05))
  (bind _returnvalue_5 (+ _worldlocation _returnvalue_4))
  (bind _intersection (Class|KismetMathLibrary|LinePlaneIntersection _worldlocation _returnvalue_5 _virtualplane))
  (switch Utilities|FlowControl|Switch|SwitchonETransformMode (Variables|Default|GetTransformMode)
    (:NewEnumerator0
      (bind _output_get (Variables|Default|SetCurrentFrameDragLocation _intersection))
      (CallFunction|TranslateObject (Variables|Default|GetConstraintAxis) (- _output_get (Variables|Default|GetPreviousFrameDragLocation)))
      (Variables|Default|SetPreviousFrameDragLocation (Variables|Default|GetCurrentFrameDragLocation))
      (return false))
    (:NewEnumerator1
      (Variables|Default|SetCurrentFrameDragLocation _intersection)
      (switch Utilities|FlowControl|Switch|SwitchonEConstraintAxis (Variables|Default|GetConstraintAxis)
        (:NewEnumerator0
          (CallFunction|RotateObject _constraintaxis (CallFunction|CalculateArcballAngleAroundAxis "NewEnumerator0" (- (Variables|Default|GetPreviousFrameDragLocation) _returnvalue_3) (- (Variables|Default|GetCurrentFrameDragLocation) _returnvalue_3))))
        (:NewEnumerator1
          (CallFunction|RotateObject _constraintaxis (CallFunction|CalculateArcballAngleAroundAxis "NewEnumerator1" (- (Variables|Default|GetPreviousFrameDragLocation) _returnvalue_3) (- (Variables|Default|GetCurrentFrameDragLocation) _returnvalue_3))))
        (:NewEnumerator2
          (CallFunction|RotateObject _constraintaxis (CallFunction|CalculateArcballAngleAroundAxis "NewEnumerator2" (- (Variables|Default|GetPreviousFrameDragLocation) _returnvalue_3) (- (Variables|Default|GetCurrentFrameDragLocation) _returnvalue_3))))
        (:NewEnumerator8
          _))
      (Variables|Default|SetPreviousFrameDragLocation (Variables|Default|GetCurrentFrameDragLocation))
      (return false))
    (:NewEnumerator2
      (CallFunction|ResizeObject (Math|Conversions|ToVector(Float) (* (+ _deltax _deltay) 0.1))))))

(fn OnTraceEnter
  (params (Interactor :type BPC%20Toolkit%20Trace%20Interactor%20Object%20Reference) (TraceHit :type Hit%20Result%20Structure%20%28by%20ref%29))
  (return false))

(fn OnTraceLeave
  (params (Interactor :type BPC%20Toolkit%20Trace%20Interactor%20Object%20Reference) (TraceHit :type Hit%20Result%20Structure%20%28by%20ref%29))
  (return false))

(fn OnTraceMove
  (params (Interactor :type BPC%20Toolkit%20Trace%20Interactor%20Object%20Reference) (TraceHit :type Hit%20Result%20Structure%20%28by%20ref%29))
  (return false))
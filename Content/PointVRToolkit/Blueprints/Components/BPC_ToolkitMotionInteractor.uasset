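; VR hand component that drives hover, grab, use and drag interaction with actors implementing BPI_ToolkitMotionInteractive.
; While active, Tick picks the nearest interactive component overlapping the hover shape and sends enter, move and leave messages on actor and component.
; Grab and use events forward to the hovered actor, whose replies set grabbing and per-tick dragging.
; A hover lock freezes target selection, and losing the target releases the grab.
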(event Custom|SetupInteractor
  (params (OverlapShape :type Primitive%20Component%20Object%20Reference))
  ;[1 1 0] 设置碰撞组件
  ;;[1 1 0] 并不知道这一步到底有没有用,我只是想在更换手部碰撞体的时候停止Tick后续执行
  (if (Variables|Default|GetbIsInteractionActivated)
    (CallFunction|DeactivateInteraction))
  (Variables|InteractorSettings|SetHoverShape OverlapShape)
  (CallFunction|ActivateInteraction))

(event Custom|ActivateInteraction
  ;[1 1 0] 组件交互逻辑的激活与停止
  (Variables|Default|SetbIsInteractionActivated true))

(event Custom|DeactivateInteraction
  ;[1 1 0] 组件交互逻辑的激活与停止
  (Variables|Default|SetbIsInteractionActivated false)
  (CallFunction|GrabReleased)
  (Class|BPIToolkitMotionInteractive|OnComponentUnhovered(Message) (Variables|HoveredObject|GetHoveredActor) self (Variables|HoveredObject|GetHoveredComponent))
  (Variables|HoveredObject|SetHoveredComponent 0)
  (Class|BPIToolkitMotionInteractive|OnHoverLeave(Message) (Variables|HoveredObject|GetHoveredActor) self)
  (Variables|HoveredObject|SetHoveredActor 0))

(event Custom|UsePressed
  ;[1 1 0] 使用捡起对象的功能
  (Class|BPIToolkitMotionInteractive|OnUsePressed(Message) (Variables|HoveredObject|GetHoveredActor) self))

(event Custom|UseReleased
  ;[1 1 0] 使用捡起对象的功能
  (Class|BPIToolkitMotionInteractive|OnUseReleased(Message) (Variables|HoveredObject|GetHoveredActor) self))

(event Custom|GrabPressed
  ;[1 1 0] 捡起对象
  (bind _returnvalue (Class|BPIToolkitMotionInteractive|OnGrabPressed(Message) (Variables|HoveredObject|GetHoveredActor) self))
  (Variables|Default|SetbIsGrabbing _returnvalue)
  ;[1 1 0] 拖拽物体，持续性事件
  (bind _returnvalue_2 (Class|BPIToolkitMotionInteractive|OnDragDetected(Message) (Variables|HoveredObject|GetHoveredActor) self))
  (Variables|Default|SetbIsDragging _returnvalue_2))

(event Custom|GrabReleased
  ;[1 1 0] 捡起对象
  (Class|BPIToolkitMotionInteractive|OnGrabReleased(Message) (Variables|HoveredObject|GetHoveredActor) self)
  (Variables|Default|SetbIsGrabbing false)
  ;[1 1 0] 拖拽物体，持续性事件
  (Class|BPIToolkitMotionInteractive|OnDragCanceled(Message) (Variables|HoveredObject|GetHoveredActor) self)
  (Variables|Default|SetbIsDragging false))

(event Custom|SetCustomHovered
  (params (CustomActor :type Actor%20Object%20Reference) (CustomComponent :type Primitive%20Component%20Object%20Reference) (Lock :type Boolean))
  ;[1 1 0] 这边我跟原作者不太一样，可能原作者的方法更好
  (Variables|HoveredObject|SetHoveredActor CustomActor)
  (Variables|HoveredObject|SetHoveredComponent CustomComponent)
  (if Lock
    (CallFunction|LockHovered)
    (else
      (CallFunction|UnlockHovered))))

(event Custom|LockHovered
  ;[1 1 0] 交互对象的锁定与解锁，一般用于防止手在和对象交互时被另一个对象打断
  (Variables|Default|SetbLockOnHovered true))

(event Custom|UnlockHovered
  ;[1 1 0] 交互对象的锁定与解锁，一般用于防止手在和对象交互时被另一个对象打断
  (Variables|Default|SetbLockOnHovered false))

(event EventBeginPlay
  ;[1 1 0] 在游戏开始时设置该组件从属的左右手
  (bind _asbp_toolkit_vrhand (Utilities|Casting|CastToBP_ToolkitVRHand (Components|GetOwner)))
  (Variables|InteractorSettings|SetHandType (Variables|/Game/PointVRToolkit/Blueprints/Player/VirtualReality/BP_ToolkitVRHand.BP_ToolkitVRHand_C|GetHandType _asbp_toolkit_vrhand)))

(event EventTick
  (params (DeltaSeconds :type Float%20%28single-precision%29))
  ;[1 0 0] 整个VR交互框架的核心逻辑
  (if (Variables|Default|GetbIsInteractionActivated)
    (Utilities|FlowControl|Sequence
      (:then_0
        (if (not (Variables|Default|GetbLockOnHovered))
          (bind (_outactor _outcomponent) (CallFunction|GetClosestHoveredObject)) ; 重要：这个函数虽然只有返回值但是不要改成纯函数，如果改成纯函数则在单个Tick周期内，该函数会被执行多次
          (if (== (Variables|HoveredObject|GetHoveredActor) _outactor)
            (Class|BPIToolkitMotionInteractive|OnHoverMove(Message) (Variables|HoveredObject|GetHoveredActor) self)
            (if (not (== (Variables|HoveredObject|GetHoveredComponent) _outcomponent))
              (Class|BPIToolkitMotionInteractive|OnComponentUnhovered(Message) (Variables|HoveredObject|GetHoveredActor) self (Variables|HoveredObject|GetHoveredComponent))
              (Variables|HoveredObject|SetHoveredComponent 0)
              (Class|BPIToolkitMotionInteractive|OnComponentHovered(Message) (Variables|HoveredObject|GetHoveredActor) self _outcomponent)
              (Variables|HoveredObject|SetHoveredComponent _outcomponent))
            (else
              (CallFunction|GrabReleased)
              (Class|BPIToolkitMotionInteractive|OnHoverLeave(Message) (Variables|HoveredObject|GetHoveredActor) self)
              (Class|BPIToolkitMotionInteractive|OnComponentUnhovered(Message) (Variables|HoveredObject|GetHoveredActor) self (Variables|HoveredObject|GetHoveredComponent))
              (Variables|HoveredObject|SetHoveredActor 0)
              (Variables|HoveredObject|SetHoveredComponent 0)
              (Class|BPIToolkitMotionInteractive|OnHoverEnter(Message) _outactor self)
              (bind _output_get (Variables|HoveredObject|SetHoveredActor _outactor))
              (Class|BPIToolkitMotionInteractive|OnComponentHovered(Message) _output_get self _outcomponent)
              (Variables|HoveredObject|SetHoveredComponent _outcomponent)))))
      (:then_1
        (if (Variables|Default|GetbIsDragging)
          (Class|BPIToolkitMotionInteractive|OnDragMove(Message) (Variables|HoveredObject|GetHoveredActor) self))))))

(fn GetClosestHoveredObject
  (for _array_element (Class|PrimitiveComponent|GetOverlappingComponents (Variables|InteractorSettings|GetHoverShape))
    (if (Utilities|DoesObjectImplementInterface (Components|GetOwner _array_element) "/Game/PointVRToolkit/Blueprints/Interfaces/BPI_ToolkitMotionInteractive.BPI_ToolkitMotionInteractive_C") ; 碰到的对象是否实现了交互接口
      (bind _returnvalue (Class|BPIToolkitMotionInteractive|IsInteractiveComponent(Message) (Components|GetOwner _array_element) self _array_element))
      (if _returnvalue ; 碰到的组件是否可交互
        (LocalVariables|SetTempActor (Components|GetOwner _array_element))
        (bind _output_get (LocalVariables|SetTempComponent _array_element))
        (if (< (.ReturnValue (Collision|GetClosestPointonCollision _output_get (Transformation|GetWorldLocation (Variables|InteractorSettings|GetHoverShape)) "None")) (LocalVariables|GetClosestDistance)) ; 这个组件和手的距离是否小于上一个距离
          (LocalVariables|SetClosestDistance (.ReturnValue (Collision|GetClosestPointonCollision _output_get (Transformation|GetWorldLocation (Variables|InteractorSettings|GetHoverShape)) "None")))
          (LocalVariables|SetClosestComponent (LocalVariables|GetTempComponent))
          (LocalVariables|SetClosestActor (LocalVariables|GetTempActor))))))
  (return (LocalVariables|GetClosestActor) (LocalVariables|GetClosestComponent)))

(fn GetHand
  (return (Variables|InteractorSettings|GetHandType)))

(fn GetHoveredObject
  (return (Variables|HoveredObject|GetHoveredActor) (Variables|HoveredObject|GetHoveredComponent)))

(fn GetHoverShape
  (return (Variables|InteractorSettings|GetHoverShape)))
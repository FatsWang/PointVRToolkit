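; Blueprint function library of actor utilities for the PointVR Toolkit, covering attachment hierarchy queries and scale changes.
; GetAllAttachedActors returns every descendant of a root actor through a recursive helper that walks the attachment tree depth-first, adding each child before its own children.
; AddActorWorldScale3D adds a delta to an actor's scale per axis, clamping each component to a small positive minimum and a large maximum.
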(fn GetAllAttachedActors
  (params (RootActor :type Actor%20Object%20Reference))
  (bind _attachedactors (LocalVariables|GetAttachedActors))
  (CallFunction|GetAllAttachedActorsRecursively RootActor _attachedactors)
  (return _attachedactors))

(fn GetAllAttachedActorsRecursively
  (params (RootActor :type Actor%20Object%20Reference) (AttachedActors :type Array%20of%20Actor%20Object%20References))
  (for _array_element (Actor|GetAttachedActors RootActor)
    (Utilities|FlowControl|Sequence
      (:then_0
        (Utilities|Array|Add AttachedActors _array_element))
      (:then_1
        (CallFunction|GetAllAttachedActorsRecursively _array_element AttachedActors)))))

(fn AddActorWorldScale3D
  (params (Actor :type Actor%20Object%20Reference) (DeltaScale :type Vector))
  (bind _returnvalue (Transformation|GetActorScale3D Actor))
  (Transformation|SetActorScale3D Actor (Math|Vector|MakeVector (Math|Float|Clamp(Float) (+ (.x _returnvalue) (.x DeltaScale)) 0.001 1e+03) (Math|Float|Clamp(Float) (+ (.y _returnvalue) (.y DeltaScale)) 0.001 1e+03) (Math|Float|Clamp(Float) (+ (.z _returnvalue) (.z DeltaScale)) 0.001 1e+03))))